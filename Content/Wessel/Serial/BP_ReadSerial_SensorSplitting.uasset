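; Serial sensor router that turns readings from two hand scanners, four valves and four dials into in-game control states.
; GetDataFromSensors routes readings by ID, pressing scanners or filling valve and dial angle arrays.
; On a dedicated server, Tick applies those angles and sends changed values to clients through events.
; A trigger window pairs both scanner presses, though its timeout compares frame delta times rather than elapsed world time.
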(event `Multicast_SendValveToClient`
  (params (ValveID :type Integer) (ValveValue :type Integer))
  (bind _returnvalue (`KismetMathLibrary.Conv_IntToDouble` ValveValue))
  (switch `int` ValveID
    (:`0`
      (set `/Game/Bo/Scripts/Valves/BP_Base_Valve.currentValue` _returnvalue (`self.Valve_1`)))
    (:`1`
      (set `/Game/Bo/Scripts/Valves/BP_Base_Valve.currentValue` _returnvalue (`self.Valve_2`)))
    (:`2`
      (set `/Game/Bo/Scripts/Valves/BP_Base_Valve.currentValue` _returnvalue (`self.Valve_3`)))
    (:`3`
      (set `/Game/Bo/Scripts/Valves/BP_Base_Valve.currentValue` _returnvalue (`self.Valve_4`)))))

(event `SendKnobValueToClient`
  (params (KnobID :type Integer) (KnobValue :type Integer))
  (bind _returnvalue (`KismetMathLibrary.Conv_IntToDouble` KnobValue))
  (switch `int` KnobID
    (:`0`
      (set `/Game/Bo/Scripts/Pillars/BP_Base_Knob.currentValue` _returnvalue (`self.Knob_1`)))
    (:`1`
      (set `/Game/Bo/Scripts/Pillars/BP_Base_Knob.currentValue` _returnvalue (`self.Knob_2`)))
    (:`2`
      (set `/Game/Bo/Scripts/Pillars/BP_Base_Knob.currentValue` _returnvalue (`self.Knob_3`)))
    (:`3`
      (set `/Game/Bo/Scripts/Pillars/BP_Base_Knob.currentValue` _returnvalue (`self.Knob_4`)))))

(event `self.ReceiveTick`
  (params (DeltaSeconds :type "Float (single-precision)"))
  (bind _output (`|GetArrayItem` (`self.ValveAngles`) 3))
  (bind _output_2 (`|GetArrayItem` (`self.ValveAngles`)))
  (bind _output_3 (`|GetArrayItem` (`self.ButtonAngles`)))
  (bind _output_4 (`|GetArrayItem` (`self.ButtonAngles`) 1))
  (bind _output_5 (`|GetArrayItem` (`self.ButtonAngles`) 2))
  (bind _output_6 (`|GetArrayItem` (`self.ButtonAngles`) 3))
  (bind _output_7 (`|GetArrayItem` (`self.ValveAngles`) 1))
  (bind _output_8 (`|GetArrayItem` (`self.ValveAngles`) 2))
  (if (`KismetSystemLibrary.IsDedicatedServer`)
    (`|ExecutionSequence`
      (:`then_0`
        ;[1 1 1] Outputs Bool: HandscannersSet
        (if (not (`self.Handscanners Set`))
          (`self.BothHandScannersPressedWithinTimeLimit` (`self.TriggerWindowDuration`))))
      (:`then_1`
        (`|ExecutionSequence`
          (:`then_0`
            ;[1 1 1] Set Valve Rotation and send to client
            (if (not (== _output_2 (`self.PreviousValveValue_1`)))
              (`KismetSystemLibrary.PrintString` "1 Differnet from previous value")
              (`self.Multicast_SendValveToClient` 0 _output_2))
            (set `/Game/Bo/Scripts/Valves/BP_Base_Valve.currentValue` (`KismetMathLibrary.Conv_IntToDouble` _output_2) (`self.Valve_1`))
            (set `self.PreviousValveValue_1` _output_2))
          (:`then_1`
            (if (not (== _output_7 (`self.PreviousValveValue_2`)))
              (`KismetSystemLibrary.PrintString` "2 Differnet from previous value")
              (`self.Multicast_SendValveToClient` 1 _output_7))
            (set `/Game/Bo/Scripts/Valves/BP_Base_Valve.currentValue` (`KismetMathLibrary.Conv_IntToDouble` _output_7) (`self.Valve_2`))
            (set `self.PreviousValveValue_2` _output_7))
          (:`then_2`
            (if (not (== _output_8 (`self.PreviousValveValue_3`)))
              (`KismetSystemLibrary.PrintString` "3 Differnet from previous value")
              (`self.Multicast_SendValveToClient` 2 _output_8))
            (set `/Game/Bo/Scripts/Valves/BP_Base_Valve.currentValue` (`KismetMathLibrary.Conv_IntToDouble` _output_8) (`self.Valve_3`))
            (set `self.PreviousValveValue_3` _output_8))
          (:`then_3`
            (if (not (== _output (`self.PreviousValveValue_4`)))
              (`KismetSystemLibrary.PrintString` "4 Differnet from previous value")
              (`self.Multicast_SendValveToClient` 3 _output))
            (set `/Game/Bo/Scripts/Valves/BP_Base_Valve.currentValue` (`KismetMathLibrary.Conv_IntToDouble` _output) (`self.Valve_4`))
            (set `self.PreviousValveValue_4` _output))
          (:`then_4`
            (`|ExecutionSequence`
              (:`then_0`
                (if (not (== _output_3 (`self.PreviousKnobValue_1`)))
                  (`KismetSystemLibrary.PrintString` "5 Differnet from previous value")
                  (`self.SendKnobValueToClient` 0 _output_3))
                (set `/Game/Bo/Scripts/Pillars/BP_Base_Knob.currentValue` (`KismetMathLibrary.Conv_IntToDouble` _output_3) (`self.Knob_1`))
                (set `self.PreviousKnobValue_1` _output_3))
              (:`then_1`
                (if (not (== _output_4 (`self.PreviousKnobValue_2`)))
                  (`KismetSystemLibrary.PrintString` "6 Differnet from previous value")
                  (`self.SendKnobValueToClient` 1 _output_4))
                (set `/Game/Bo/Scripts/Pillars/BP_Base_Knob.currentValue` (`KismetMathLibrary.Conv_IntToDouble` _output_4) (`self.Knob_2`))
                (set `self.PreviousKnobValue_2` _output_4))
              (:`then_2`
                (if (not (== _output_5 (`self.PreviousKnobValue_3`)))
                  (`KismetSystemLibrary.PrintString` "7 Differnet from previous value")
                  (`self.SendKnobValueToClient` 2 _output_5))
                (set `/Game/Bo/Scripts/Pillars/BP_Base_Knob.currentValue` (`KismetMathLibrary.Conv_IntToDouble` _output_5) (`self.Knob_3`))
                (set `self.PreviousKnobValue_3` _output_5))
              (:`then_3`
                (if (not (== _output_6 (`self.PreviousKnobValue_4`)))
                  (`KismetSystemLibrary.PrintString` "8 Differnet from previous value")
                  (`self.SendKnobValueToClient` 3 _output_6))
                (set `/Game/Bo/Scripts/Pillars/BP_Base_Knob.currentValue` (`KismetMathLibrary.Conv_IntToDouble` _output_6) (`self.Knob_4`))
                (set `self.PreviousKnobValue_4` _output_6)))))))))

(event `GetDataFromSensors`
  (params (SensorID :type Integer) (SensorData :type Integer))
  (bind _sensorvalue (`self.SensorValue`))
  (bind _sensorvalue_2 (`self.SensorValue`))
  (bind _valveangles (`self.ValveAngles`))
  (bind _buttonangles (`self.ButtonAngles`))
  (bind _returnvalue (!= 0 (`self.SensorValue`)))
  (set `self.SensorValue` SensorData)
  (`KismetSystemLibrary.PrintString` (`KismetStringLibrary.BuildString_Int` (`KismetStringLibrary.BuildString_Int` "" "ID: " SensorID) " Data: " SensorData))
  ;[1 1 1] All locations are as if you are standing in front of them
  ; 1 = Left Handscanner
  ; 2 = Right Handscanner
  ; 3 = LeftMost Valve
  ; 4 = LeftMiddle Valve
  ; 5 = RightMiddle Valve
  ; 6 = RightMost Valve
  ; 7 = Topleft Dial
  ; 8 = TopRight Dial
  ; 9 = BottomLeft Dial
  ; 10 = BottomRIght Dial
  (switch `int` SensorID ; Don't use 0
    (:`Default`
      (`|ExecutionSequence` :!label _label
        (:`then_0`
          (`KismetSystemLibrary.PrintString` (`KismetStringLibrary.BuildString_Int` "" "ID not Recognized: " SensorID)))))
    (:`0`
      (goto _label))
    (:`1`
      (if _returnvalue
        ;[1 1 1] Outputs Bool: HandscannersSet
        (`self.Right Handscanner Set`)))
    (:`2`
      (if _returnvalue
        (`self.Left Hand Scanner Set`)))
    (:`3`
      ;[1 1 1] Set Valve values in 1 array
      (`KismetArrayLibrary.Array_Set` _valveangles 0 _sensorvalue_2))
    (:`4`
      (`KismetArrayLibrary.Array_Set` _valveangles 1 _sensorvalue_2))
    (:`5`
      (`KismetArrayLibrary.Array_Set` _valveangles 2 _sensorvalue_2))
    (:`6`
      (`KismetArrayLibrary.Array_Set` _valveangles 3 _sensorvalue_2))
    (:`7`
      ;[1 1 1] Set Dials to 1 array
      (`KismetArrayLibrary.Array_Set` _buttonangles 0 _sensorvalue))
    (:`8`
      (`KismetArrayLibrary.Array_Set` _buttonangles 1 _sensorvalue))
    (:`9`
      (`KismetArrayLibrary.Array_Set` _buttonangles 2 _sensorvalue))
    (:`10`
      (`KismetArrayLibrary.Array_Set` _buttonangles 3 _sensorvalue))))

(fn `BoMockup`)

(fn `BothHandScannersPressedWithinTimeLimit`
  (params (MaxTimeBetweenButtonsPressed :type "Float (double-precision)"))
  (if (`self.TriggerWindowActive`)
    (set `self.ElapsedTime` (`KismetMathLibrary.Abs` (- (`GameplayStatics.GetWorldDeltaSeconds`) (`self.FirstInputTime`))))
    (if (> (`self.ElapsedTime`) MaxTimeBetweenButtonsPressed)
      (`|ExecutionSequence`
        (:`then_0`
          (set `self.Left Handscanner set` false)
          (`/Game/Bo/Scripts/Handscanners/BP_Base_Handscanner.ButtonRelease` (`self.HandScannerLeft`))
          (set `self.LeftButtonOn` false))
        (:`then_1`
          (set `self.Right Handscanner` false)
          (`/Game/Bo/Scripts/Handscanners/BP_Base_Handscanner.ButtonRelease` (`self.HandScannerRight`))
          (set `self.RightButtonOn` false))
        (:`then_2`
          (set `self.TriggerWindowActive` false))))))

(fn `Left Hand Scanner Set`
  (bind _returnvalue (`GameplayStatics.GetWorldDeltaSeconds`))
  (if (not (`self.LeftButtonOn`))
    (set `self.LeftButtonOn` true)
    (`/Game/Bo/Scripts/Handscanners/BP_Base_Handscanner.PressButton` (`self.HandScannerLeft`))
    (`KismetSystemLibrary.PrintString` "Left Pressed"))
  (if (`self.TriggerWindowActive`)
    (set `self.Left Handscanner set` true)
    (if (`self.Right Handscanner`)
      (set `self.Handscanners Set` true)
      (set `self.TriggerWindowActive` false)
      (else
        (set `self.FirstInputTime` _returnvalue)))
    (else
      (set `self.Left Handscanner set` true)
      (set `self.TriggerWindowActive` true)
      (set `self.FirstInputTime` _returnvalue))))

(fn `Right Handscanner Set`
  (bind _returnvalue (`GameplayStatics.GetWorldDeltaSeconds`))
  (if (not (`self.RightButtonOn`))
    (set `self.RightButtonOn` true)
    (`/Game/Bo/Scripts/Handscanners/BP_Base_Handscanner.PressButton` (`self.HandScannerRight`))
    (`KismetSystemLibrary.PrintString` "Right hand press"))
  (if (`self.TriggerWindowActive`)
    (set `self.Right Handscanner` true)
    (if (`self.Left Handscanner set`)
      (set `self.Handscanners Set` true)
      (set `self.TriggerWindowActive` false)
      (else
        (set `self.FirstInputTime` _returnvalue)))
    (else
      (set `self.Right Handscanner` true)
      (set `self.TriggerWindowActive` true)
      (set `self.FirstInputTime` _returnvalue))))

(fn `UserConstructionScript`)