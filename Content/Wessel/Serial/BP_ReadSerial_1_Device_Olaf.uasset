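; Serial bridge that feeds Arduino sensor readings into the game and can trigger the Arduino's lift sequence.
; On a dedicated server, BeginPlay scans COM ports, keeps the last one opened and starts a per-tick request-and-read loop.
; A byte counter assembles four-byte frames into a sensor ID and signed 16-bit value for ReadSerialSensor, discarding the last byte.
; EndPlay closes the stored port to keep port numbering stable.
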(event `self.ReceiveBeginPlay`
  ;[0.3005 0.3005 0.3005 1 30] START
  (if (`KismetSystemLibrary.IsDedicatedServer`)
    ;[0.3005 0.3005 0.3005] ENABLE KEYBOARD INPUT (DEBUG)
    (`self.EnableInput` (`GameplayStatics.GetPlayerController` 0))
    ;[0.3005 0.3005 0.3005 1 40] OPEN SERIAL PORTS - Will throw errors for each port without a connection
    (bind _index (`/Game/EditorBlueprintResources/StandardMacros.ForLoop` 0 255)
      (:`LoopBody`
        (bind (_bopened _returnvalue) (`SerialCom.OpenComPortWithFlowControl` _index 115200))
        (if _bopened
          (`SerialCom.Flush` _returnvalue)
          (set `self.MySerialPort` _returnvalue)
          (else
            (`SerialCom.Close` _returnvalue))))
      (:`Completed`
        (`KismetSystemLibrary.PrintString` "SETUP DONE")
        (`self.RequestData`)))))

(event `self.ReceiveEndPlay`
  (params (EndPlayReason :type "EEndPlayReason Enum" :default "Destroyed"))
  (bind _myserialport (`self.MySerialPort`))
  ;[0.3005 0.3005 0.3005 1 40] Close a port before quitting, otherwise your ports will be different next time
  (if (`KismetSystemLibrary.IsDedicatedServer`)
    _
    (else
      _))
  (`SerialCom.Close` _myserialport)
  (`KismetSystemLibrary.PrintString` "Closed port: ")
  (`KismetSystemLibrary.PrintString` (`KismetSystemLibrary.GetDisplayName` _myserialport)))

(event `RequestData`
  (bind _currentbyte (`self.CurrentByte`))
  ;[0.302 0.302 0.302] Write Request to Arduino
  (`SerialCom.WriteByte` (`self.MySerialPort`) 255)
  (if true
    ;[0.3005 0.3005 0.3005 1 40] Read from port every frame
    (`/Game/EditorBlueprintResources/StandardMacros.ForLoop` 0 3
      (:`LoopBody`
        (bind (_bsuccess _returnvalue) (`SerialCom.ReadByte` (`self.MySerialPort`)))
        (if _bsuccess
          ;[0.3005 0.3005 0.3005 1 40] Math to make 3 Bytes into an ID Int and a SensorValue Int
          (set `self.CurrentByte` (`KismetMathLibrary.Conv_ByteToInt` _returnvalue))
          (switch `int` (`self.ByteCounter`)
            (:`0`
              (set `self.ByteCounter` 1)
              (set `self.SensorID` _currentbyte))
            (:`1`
              (set `self.ByteCounter` 2)
              (bind _output_get (set `self.SensorMSByte` _currentbyte)))
            (:`2`
              (set `self.ByteCounter` 3)
              (bind _output_get_2 (set `self.SensorLSByte` _currentbyte))
              (bind _returnvalue_2 (`KismetMathLibrary.Or_IntInt` (* _output_get 256) _output_get_2))
              (if (!= (`KismetMathLibrary.And_IntInt` _returnvalue_2 32768) 0)
                (set `self.SensorValue` (- _returnvalue_2 65536))
                (else
                  (set `self.SensorValue` _returnvalue_2)))
              (`/Game/Wessel/Serial/BP_ReadSerial_SensorSplitting.GetDataFromSensors` (`self.ReadSerialSensor`) (`self.SensorID`) (`self.SensorValue`)))
            (:`3`
              (set `self.ByteCounter` 0)))))
      (:`Completed`
        (`KismetSystemLibrary.DelayUntilNextTick`)
        (`self.RequestData`)))))

(event `StartArduinoLiftSequence`
  (`SerialCom.WriteByte` (`self.MySerialPort`) 254))

(fn `UserConstructionScript`)