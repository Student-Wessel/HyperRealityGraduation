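; Client-side elevator transition that lifts a list of actors, plus OnlineTrackedPawns, from the Below to the Above dynamic level.
; MoveUp opens tagged shutters, gathers the pawns, then starts the transition.
; Tick offsets everything upward until a reference actor reaches the switch height, where movement pauses for a blocking stream-level swap.
; Movement then resumes to the final height while remaining shutters open and are destroyed after delays.
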(event `self.ReceiveTick`
  (params (DeltaSeconds :type "Float (single-precision)"))
  (if (`KismetSystemLibrary.IsDedicatedServer`)
    _
    (elif (`self.SwitchingScene`)
      _
      (elif (`self.PlayTransition`)
        (if (`self.SwitchedScene`)
          (if (< (.z (`self.K2_GetActorLocation` (`self.ReferenceActor`))) (`self.FinalHeightTarget`))
            (`self.MoveActorsUp` DeltaSeconds)
            (else
              (set `self.PlayTransition` false)
              (`KismetSystemLibrary.PrintString` "Transition done")))
          (elif (< (.z (`self.K2_GetActorLocation` (`self.ReferenceActor`))) (`self.SceneSwitchHeight`))
            (`self.MoveActorsUp` DeltaSeconds)
            (else
              (set `self.SwitchingScene` true)
              (`KismetSystemLibrary.PrintString` "Loading")
              (`GameplayStatics.UnloadStreamLevelBySoftObjectPtr` "/Game/Wessel/Map/Below_Dynamic_Extended.Below_Dynamic_Extended" true)
              (`KismetSystemLibrary.PrintString` "Unloaded")
              (`KismetSystemLibrary.Delay` 1.0)
              (`GameplayStatics.LoadStreamLevelBySoftObjectPtr` "/Game/Wessel/Map/Above_Dynamic_Extended.Above_Dynamic_Extended" true true)
              (set `self.SwitchingScene` false)
              (set `self.SwitchedScene` true)
              (`KismetSystemLibrary.Delay` 3.0)
              (bind _outactors (`GameplayStatics.GetAllActorsOfClass` "/Game/Bo/Scripts/Elevator/BP_ElevatorShutters.BP_ElevatorShutters_C"))
              (for _array_element _outactors
                (`/Game/Bo/Scripts/Elevator/BP_ElevatorShutters.OpenShutters` _array_element)
                (`KismetSystemLibrary.Delay` 2.0)
                (`self.K2_DestroyActor` _array_element)))))))))

(event `MoveUp`
  (if (not (`KismetSystemLibrary.IsDedicatedServer`))
    (`KismetSystemLibrary.Delay` 1.0)
    (`KismetSystemLibrary.PrintString` "Move Up Request came through")
    (bind _outactors (`GameplayStatics.GetAllActorsWithTag` "ElevatorShutterBot"))
    (for _array_element _outactors
      (if (`KismetSystemLibrary.IsValid` _array_element)
        (bind _asbp_elevator_shutters (cast `/Game/Bo/Scripts/Elevator/BP_ElevatorShutters` _array_element))
        (`/Game/Bo/Scripts/Elevator/BP_ElevatorShutters.OpenShutters` _asbp_elevator_shutters)))
    (`KismetSystemLibrary.Delay` 4.0)
    (bind _outactors_2 (`GameplayStatics.GetAllActorsOfClass` "/Game/OculusRetargeting/UnrealManequin/OnlineTrackedPawn.OnlineTrackedPawn_C"))
    (bind _output_get (set `self.Pawns` _outactors_2))
    (if (`self.AddedPawnsToActors`)
      (set `self.PlayTransition` true)
      (`KismetSystemLibrary.PrintString` "Play transitio on")
      (else
        (for _array_element_2 _output_get
          (`KismetArrayLibrary.Array_Insert` (`self.ActorsToMove`) _array_element_2)
          (set `self.AddedPawnsToActors` true)
          (set `self.PlayTransition` true)
          (`KismetSystemLibrary.PrintString` "Play transitio on"))))))

(fn `MoveActorsUp`
  (params (DeltaTime :type "Float (double-precision)"))
  (for _array_element (`self.ActorsToMove`)
    (`self.K2_AddActorWorldOffset` _array_element (* (* (`KismetMathLibrary.MakeVector` 0.0 0.0 1.0) (`self.MoveSpeed`)) DeltaTime) false false)))

(fn `UserConstructionScript`)