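; TestPuzzle is a prototype Blueprint for a screen-based puzzle, currently holding debug and disconnected logic.
; BeginPlay prints debug labels for an array's last index and maximum value.
; A self-recalling PrintRandomInt event prints a random integer on a half-second delay, but its only outside call is unwired.
; Unwired chains set Screen material scalar parameters for five "Correct" indicators and an emissive switch, while Tick and the construction script are empty.
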(event `self.ReceiveBeginPlay`
  (`KismetSystemLibrary.PrintString` (`KismetStringLibrary.BuildString_Int` "" "last index: " (`KismetArrayLibrary.Array_LastIndex` (`self.Array`))))
  (`KismetSystemLibrary.PrintString` (`KismetStringLibrary.BuildString_Int` "" "index of maxe value: "))
  (`KismetSystemLibrary.PrintString` (`KismetStringLibrary.BuildString_Int` "" "max value: ")))

(event `self.ReceiveTick`
  (params (DeltaSeconds :type "Float (single-precision)")))

(event `PrintRandomInt`
  (`KismetSystemLibrary.PrintString` (`KismetStringLibrary.Conv_IntToString` (`KismetMathLibrary.RandomInteger` 3)))
  (`KismetSystemLibrary.Delay` 0.5)
  (`self.PrintRandomInt`))

(fn `UserConstructionScript`)