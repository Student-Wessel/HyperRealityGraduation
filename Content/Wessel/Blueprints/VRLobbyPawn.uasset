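; VR lobby pawn that starts in Meta Quest passthrough and connects the player to a hardcoded LAN server through a gesture.
; BeginPlay initializes persistent passthrough and suppresses the boundary after a short delay.
; Each Tick, holding the right controller near headset height fades passthrough out, otherwise it fades back in.
; Once nearly transparent, passthrough is destroyed and the server's IP is opened as a level.
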(event `self.ReceiveBeginPlay`
  (bind _returnvalue (`OculusXRPassthroughSubsystem.InitializePersistentPassthrough` :`self` (subsystem `OculusXRPassthroughSubsystem`)))
  (set `self.PassthroughOpacity` (`OculusXRPassthroughLayerBase.TextureOpacityFactor` (`OculusXRPersistentPassthroughInstance.GetShape` _returnvalue)))
  (`KismetSystemLibrary.Delay` 3.0)
  (`OculusXRSceneFunctionLibrary.RequestBoundaryVisibility` "Suppressed"))

(event `self.ReceiveTick`
  (params (DeltaSeconds :type "Float (single-precision)"))
  (bind _passthroughopacity (`self.PassthroughOpacity`))
  (bind _returnvalue (* DeltaSeconds (`self.FadeSpeedFactor`)))
  (bind _returnvalue_2 (`OculusXRPersistentPassthroughInstance.GetShape` (`OculusXRPassthroughSubsystem.GetPersistentPassthrough` (subsystem `OculusXRPassthroughSubsystem`))))
  (bind _returnvalue_3 (- _passthroughopacity _returnvalue))
  (bind _returnvalue_4 (+ _passthroughopacity _returnvalue))
  (if (`KismetMathLibrary.NearlyEqual_FloatFloat` (.z (`SceneComponent.K2_GetComponentLocation` (`self.Camera`))) (.z (`SceneComponent.K2_GetComponentLocation` (`self.MotionControllerRight`))) 20.0)
    (`OculusXRPassthroughLayerBase.SetTextureOpacity` _returnvalue_2 _returnvalue_3)
    (set `self.PassthroughOpacity` _returnvalue_3)
    (if (< (`self.PassthroughOpacity`) 0.05)
      (`OculusXRPassthroughSubsystem.DestroyPersistentPassthrough` (subsystem `OculusXRPassthroughSubsystem`))
      (`KismetSystemLibrary.Delay` 0.5)
      (`GameplayStatics.OpenLevel` "192.168.5.74:7777"))
    (else
      (`OculusXRPassthroughLayerBase.SetTextureOpacity` _returnvalue_2 _returnvalue_4)
      (set `self.PassthroughOpacity` (`KismetMathLibrary.FClamp` _returnvalue_4)))))

(fn `UserConstructionScript`)