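; Long shutter actor that slides upward to open when its OpenShutters event is called, then removes itself.
; On non-dedicated-server instances only, a timeline lerps the shutter's world location from the scene root to a point above it, then destroys the actor after a short delay.
; A dedicated server only prints a debug message, without moving or destroying it.
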(event `self.OpenShutters`
  (bind (_returnvalue_x _returnvalue_y _returnvalue_z) (`KismetMathLibrary.BreakVector` (`SceneComponent.K2_GetComponentLocation` (`self.DefaultSceneRoot`))))
  (`KismetSystemLibrary.PrintString` "Called")
  (if (not (`KismetSystemLibrary.IsDedicatedServer`))
    (bind (_direction _newtrack_0) (`Timeline|Timeline` :!via `PlayFromStart`)
      (:`Update`
        (`SceneComponent.K2_SetWorldLocation` (`self.Shutters_long`) (`KismetMathLibrary.VLerp` (`SceneComponent.K2_GetComponentLocation` (`self.DefaultSceneRoot`)) (`KismetMathLibrary.MakeVector` _returnvalue_x _returnvalue_y (+ _returnvalue_z 200.0)) _newtrack_0) false false))
      (:`Finished`
        (`KismetSystemLibrary.Delay` 1.0)
        (`self.K2_DestroyActor`)))))

(fn `UserConstructionScript`)