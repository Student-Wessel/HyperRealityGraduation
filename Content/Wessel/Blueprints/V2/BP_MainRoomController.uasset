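; Controls the main room of a networked underwater VR puzzle experience, covering hand scanners, valves, knobs, lighting and audio.
; The dedicated server tracks puzzle inputs, with either scanner opening shutters and resetting ceiling lights through multicasts; valve and knob success only set flags.
; Clients run creaking, alarm and voice lines chained by audio-finished events, ending in an Arduino lift sequence.
; Several power-up and two-hand scanner chains are left unconnected.
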(event `Underwater Creaking`
  (bind _returnvalue (`KismetMathLibrary.RandomFloatInRange` 0.0 8.0))
  ;[0.3672 0.7867 1] SFX_Underwater_Creaking
  (if (not (`self.LockIsShot`))
    (`KismetSystemLibrary.RetriggerableDelay` _returnvalue)
    (switch `int` (`KismetMathLibrary.RandomInteger` 8)
      (:`Default`
        (`KismetSystemLibrary.Delay` _returnvalue)
        (`self.Underwater Creaking` :!label _label))
      (:`0`
        (`AudioComponent.Play` (`self.SFX_Creaking0`) 0.0))
      (:`1`
        (`AudioComponent.Play` (`self.SFX_Creaking1`) 0.0))
      (:`2`
        (`AudioComponent.Play` (`self.SFX_Creaking2`) 0.0))
      (:`3`
        (`AudioComponent.Play` (`self.SFX_Creaking3`) 0.0))
      (:`4`
        (`AudioComponent.Play` (`self.SFX_Creaking4`) 0.0))
      (:`5`
        (`AudioComponent.Play` (`self.SFX_Creaking5`) 0.0))
      (:`6`
        (`AudioComponent.Play` (`self.SFX_Creaking6`) 0.0))
      (:`7`
        (`AudioComponent.Play` (`self.SFX_Creaking7`) 0.0)))))

(event `self.SFX_Creaking0.OnAudioFinished`
  ;[0.3672 0.7867 1] SFX_Underwater_Creaking
  (goto _label))

(event `self.SFX_Creaking1.OnAudioFinished`
  ;[0.3672 0.7867 1] SFX_Underwater_Creaking
  (goto _label))

(event `self.SFX_Creaking2.OnAudioFinished`
  ;[0.3672 0.7867 1] SFX_Underwater_Creaking
  (goto _label))

(event `self.SFX_Creaking3.OnAudioFinished`
  ;[0.3672 0.7867 1] SFX_Underwater_Creaking
  (goto _label))

(event `self.SFX_Creaking4.OnAudioFinished`
  ;[0.3672 0.7867 1] SFX_Underwater_Creaking
  (goto _label))

(event `self.SFX_Creaking5.OnAudioFinished`
  ;[0.3672 0.7867 1] SFX_Underwater_Creaking
  (goto _label))

(event `self.SFX_Creaking6.OnAudioFinished`
  ;[0.3672 0.7867 1] SFX_Underwater_Creaking
  (goto _label))

(event `self.SFX_Creaking7.OnAudioFinished`
  ;[0.3672 0.7867 1] SFX_Underwater_Creaking
  (goto _label))

(event `Multicast_KnobsDone`
  ;[0.5035 0.4828 1] VOC_Sequence + LIFT
  (`AudioComponent.Play` (`self.VOC_SonarReboot`) 0.0))

(event `self.VOC_SonarReboot.OnAudioFinished`
  ;[0.5035 0.4828 1] VOC_Sequence + LIFT
  (`KismetSystemLibrary.Delay` 0.0)
  (`AudioComponent.Play` (`self.VOC_LargeObjectDetected`) 0.9) ; +0.9s to avoid double saying "ALERT"
)

(event `RetrieveLockIsShot`
  ;[0.5035 0.4828 1] VOC_Sequence + LIFT
  (bind _output_get (set `self.LockIsShot` true)))

(event `self.VOC_LargeObjectDetected.OnAudioFinished`
  ;[0.5035 0.4828 1] VOC_Sequence + LIFT
  (if (!= (stale `RetrieveLockIsShot` _output_get) true) :!label _label_2
    (`AudioComponent.Play` (`self.VOC_ForSafetyPlease`) 0.0)
    (`KismetSystemLibrary.Delay` 8.0)
    (goto _label_2)
    (else
      (`AudioComponent.Play` (`self.VOC_PleaseRemainStill`) 0.0))))

(event `self.VOC_PleaseRemainStill.OnAudioFinished`
  ;[0.5035 0.4828 1] VOC_Sequence + LIFT
  (bind _returnvalue (`GameplayStatics.GetActorOfClass` "/Game/Wessel/Serial/BP_ReadSerial_1_Device_Olaf.BP_ReadSerial_1_Device_Olaf_C"))
  (`/Game/Wessel/Serial/BP_ReadSerial_1_Device_Olaf.StartArduinoLiftSequence` _returnvalue))

(event `KnobsSucceeded`
  (if (not (`self.KnobsPassed`))
    (set `self.KnobsPassed` true)))

(event `self.VOC_SystemReboot.OnAudioFinished`
  ;[0.3761 0.3051 1] VOC_SystemReboot
  (`AudioComponent.SetVolumeMultiplier` (`self.SFX_InitialAlarm`) 1.0))

(event `SystemReboot`
  ;[0.3761 0.3051 1] VOC_SystemReboot
  (`AudioComponent.Play` (`self.VOC_SystemReboot`) 0.0))

(event `ValveSucceeded`
  (if (not (`self.ValvePassed`))
    (set `self.ValvePassed` true)))

(event `Initial Alarm`
  ;[0.3761 0.3051 1] Initial Alarm
  (if (not (`self.HandScannerPassed`))
    (`AudioComponent.Play` (`self.SFX_InitialAlarm`) 0.1)))

(event `self.SFX_InitialAlarm.OnAudioFinished`
  ;[0.3761 0.3051 1] Initial Alarm
  (`self.Initial Alarm`))

(event `HandScannerSucceeded`
  (if (not (`self.HandScannerPassed`))
    (set `self.HandScannerPassed` true)
    (`|ExecutionSequence`
      (:`then_0`
        (`self.Multicast_OpenShuttersOnClient`))
      (:`then_1`
        (`self.Multicast_SetCeilingLightsClients`)))))

(event `self.ReceiveBeginPlay`
  (bind _handscanner_l (`self.HandScanner_L`))
  (bind _handscanner_r (`self.HandScanner_R`))
  (`|ExecutionSequence`
    (:`then_0`
      (if (`KismetSystemLibrary.IsDedicatedServer`)
        (add `/Game/Bo/Scripts/Handscanners/BP_Base_Handscanner.ButtonPress` _handscanner_l (delegate `LeftButtonPress`))
        (add `/Game/Bo/Scripts/Handscanners/BP_Base_Handscanner.ButtonRelease` _handscanner_l (delegate `LeftButtonRelease`))
        (add `/Game/Bo/Scripts/Handscanners/BP_Base_Handscanner.ButtonPress` _handscanner_r (delegate `RightButtonPress`))
        (add `/Game/Bo/Scripts/Handscanners/BP_Base_Handscanner.ButtonRelease` _handscanner_r (delegate `RightButtonRelease`))))
    (:`then_1`
      (if (`KismetSystemLibrary.IsDedicatedServer`)
        (add `/Game/Bo/Scripts/Valves/BP_Base_Valve.ValveCorrectUpdate` (`self.Valve_1`) (delegate `Valve1Update`))
        (add `/Game/Bo/Scripts/Valves/BP_Base_Valve.ValveCorrectUpdate` (`self.Valve_2`) (delegate `Valve2Update`))
        (add `/Game/Bo/Scripts/Valves/BP_Base_Valve.ValveCorrectUpdate` (`self.Valve_3`) (delegate `Valve3Update`))
        (add `/Game/Bo/Scripts/Valves/BP_Base_Valve.ValveCorrectUpdate` (`self.Valve_4`) (delegate `Valve4Update`))
        (add `/Game/Bo/Scripts/Pillars/BP_Base_Knob.ValueCorrectUpdate` (`self.Knob_1`) (delegate `Knob1Update`))
        (add `/Game/Bo/Scripts/Pillars/BP_Base_Knob.ValueCorrectUpdate` (`self.Knob_2`) (delegate `Knob2Update`))
        (add `/Game/Bo/Scripts/Pillars/BP_Base_Knob.ValueCorrectUpdate` (`self.Knob_3`) (delegate `Knob3Update`))
        (add `/Game/Bo/Scripts/Pillars/BP_Base_Knob.ValueCorrectUpdate` (`self.Knob_4`) (delegate `Knob4Update`))))
    (:`then_2`
      ;[1 1 1] Everything
      (`KismetSystemLibrary.Delay` 15.0))
    (:`then_3`
      ;[0 0.143 1] Start of SFX & VOC
      (if (not (`KismetSystemLibrary.IsDedicatedServer`))
        (`self.Underwater Creaking`)
        (`self.Initial Alarm`)
        (`KismetSystemLibrary.Delay` 4.0) ; Wait for a bit for the users to get aclimated to VR before bombarding them with VOC
        (`self.SystemReboot`)))))

(event `LeftButtonPress`
  (`self.HandScannerSucceeded`))

(event `LeftButtonRelease`)

(event `RightButtonPress`
  (`self.HandScannerSucceeded`))

(event `RightButtonRelease`)

(event `Multicast_OpenShuttersOnClient`
  (if (not (`KismetSystemLibrary.IsDedicatedServer`))
    (`/Game/Wessel/Blueprints/V2/BP_Shutter.OpenShutters` (`self.ShortShutter`))
    (`/Game/Wessel/Blueprints/V2/BP_Shutter.OpenShutters` (`self.LongShutter`))
    ;[0.6185 0.6503 1] SFX_Raise_Shutters
    (`AudioComponent.Play` (`self.SFX_RaiseShutters`) 0.0)))

(event `self.SFX_RaiseShutters.OnAudioFinished`
  ;[0.6185 0.6503 1] VOC_Raise_Shutters
  (`KismetSystemLibrary.Delay` 3.0)
  (`AudioComponent.Play` (`self.SFX_RaiseShutters`) 0.0))

(event `Multicast_TurnPipeGreen`
  (params (Index :type Integer))
  (if (not (`KismetSystemLibrary.IsDedicatedServer`))
    (switch `int` Index
      (:`0`
        (`MeshComponent.SetScalarParameterValueOnMaterials` (`StaticMeshActor.StaticMeshComponent` (`self.PipeLight_1`)) "Turn_Green" 1.0))
      (:`1`
        (`MeshComponent.SetScalarParameterValueOnMaterials` (`StaticMeshActor.StaticMeshComponent` (`self.PipeLight_2`)) "Turn_Green" 1.0))
      (:`2`
        (`MeshComponent.SetScalarParameterValueOnMaterials` (`StaticMeshActor.StaticMeshComponent` (`self.PipeLight_3`)) "Turn_Green" 1.0))
      (:`3`
        (`MeshComponent.SetScalarParameterValueOnMaterials` (`StaticMeshActor.StaticMeshComponent` (`self.PipeLight_4`)) "Turn_Green" 1.0)))))

(event `Multicast_SetCeilingLightsClients`
  (if (not (`KismetSystemLibrary.IsDedicatedServer`))
    (for _array_element (`self.CeilingLights`)
      (bind _staticmeshcomponent (`StaticMeshActor.StaticMeshComponent` _array_element))
      (`MeshComponent.SetScalarParameterValueOnMaterials` _staticmeshcomponent "ChangeToRed" 0.0)
      (`MeshComponent.SetScalarParameterValueOnMaterials` _staticmeshcomponent "Emisve_Intensity" 50.0))))

(event `Multicast_TurnOnPipeLights`
  (if (not (`KismetSystemLibrary.IsDedicatedServer`))
    (`MeshComponent.SetScalarParameterValueOnMaterials` (`StaticMeshActor.StaticMeshComponent` (`self.PipeLight_1`)) "Emissive_Switch" 1.0)
    (`MeshComponent.SetScalarParameterValueOnMaterials` (`StaticMeshActor.StaticMeshComponent` (`self.PipeLight_2`)) "Emissive_Switch" 1.0)
    (`MeshComponent.SetScalarParameterValueOnMaterials` (`StaticMeshActor.StaticMeshComponent` (`self.PipeLight_3`)) "Emissive_Switch" 1.0)
    (`MeshComponent.SetScalarParameterValueOnMaterials` (`StaticMeshActor.StaticMeshComponent` (`self.PipeLight_4`)) "Emissive_Switch" 1.0)
    ;[0 0.1915 1] GENERATOR ONLINE
    (`AudioComponent.Play` (`self.SFX_GeneratorStartup`) 0.0)))

(event `self.SFX_GeneratorStartup.OnAudioFinished`
  ;[0 0.1915 1] GENERATOR ONLINE
)

(event `self.SFX_GeneratorLoop.OnAudioFinished`
  ;[0 0.1915 1] GENERATOR ONLINE
  (`AudioComponent.Play` (`self.SFX_GeneratorLoop`) 0.0))

(event `Valve4Update`
  (params (IsCorrect :type Boolean))
  (`KismetArrayLibrary.Array_Set` (`self.ValveValues`) 3 IsCorrect)
  (bind _allvalvescorrect (`self.AreAllValvesCorrect` (`self.ValveValues`) :!label _label_3))
  (if _allvalvescorrect
    (`self.ValveSucceeded`)))

(event `Knob4Update`
  (params (IsCorrect :type Boolean))
  (`KismetArrayLibrary.Array_Set` (`self.KnobValues`) 3 IsCorrect)
  (bind _allknobscorrect (`self.AreAllKnobsCorrect` (`self.KnobValues`) :!label _label_4))
  (if _allknobscorrect
    (`self.KnobsSucceeded`)))

(event `Multicast_TurnOnConsols`
  (if (not (`KismetSystemLibrary.IsDedicatedServer`))
    (`MeshComponent.SetScalarParameterValueOnMaterials` (`self.Room_OnlyModel_Seperated_CollidersV3_Desk02_Screen_low`) "Emissive_Switch" 1.0)
    (`MeshComponent.SetScalarParameterValueOnMaterials` (`StaticMeshActor.StaticMeshComponent` (`self.ExternalConsoleScreen`)) "Emissive_Switch" 1.0)))

(event `Knob1Update`
  (params (IsCorrect :type Boolean))
  (`KismetArrayLibrary.Array_Set` (`self.KnobValues`) 0 IsCorrect)
  (goto _label_4))

(event `Knob2Update`
  (params (IsCorrect :type Boolean))
  (`KismetArrayLibrary.Array_Set` (`self.KnobValues`) 1 IsCorrect)
  (goto _label_4))

(event `Knob3Update`
  (params (IsCorrect :type Boolean))
  (`KismetArrayLibrary.Array_Set` (`self.KnobValues`) 2 IsCorrect)
  (goto _label_4))

(event `Multicast_TurnOnHandScanners`
  (if (not (`KismetSystemLibrary.IsDedicatedServer`))
    (`MeshComponent.SetScalarParameterValueOnMaterials` (`/Game/Bo/Scripts/Handscanners/BP_Base_Handscanner.Stuff_02_V01_low_Scanner_low` (`self.HandScanner_L`)) "Emissive_Switch" 1.0)
    (`MeshComponent.SetScalarParameterValueOnMaterials` (`/Game/Bo/Scripts/Handscanners/BP_Base_Handscanner.Stuff_02_V01_low_Scanner_low` (`self.HandScanner_R`)) "Emissive_Switch" 1.0)))

(event `Valve3Update`
  (params (IsCorrect :type Boolean))
  (`KismetArrayLibrary.Array_Set` (`self.ValveValues`) 2 IsCorrect)
  (goto _label_3))

(event `Multicast_ClientPressLeftHandScanner`
  (if (not (`KismetSystemLibrary.IsDedicatedServer`))
    (`MeshComponent.SetScalarParameterValueOnMaterials` (`/Game/Bo/Scripts/Handscanners/BP_Base_Handscanner.Stuff_02_V01_low_Scanner_low` (`self.HandScanner_L`)) "Emissive_Switch" 10.0)))

(event `Valve1Update`
  (params (IsCorrect :type Boolean))
  (`KismetArrayLibrary.Array_Set` (`self.ValveValues`) 0 IsCorrect)
  (goto _label_3))

(event `Valve2Update`
  (params (IsCorrect :type Boolean))
  (`KismetArrayLibrary.Array_Set` (`self.ValveValues`) 1 IsCorrect)
  (goto _label_3))

(event `Multicast_TurnPipeRed`
  (params (Index :type Integer))
  (if (not (`KismetSystemLibrary.IsDedicatedServer`))
    (switch `int` Index
      (:`0`
        (`MeshComponent.SetScalarParameterValueOnMaterials` (`StaticMeshActor.StaticMeshComponent` (`self.PipeLight_1`)) "Turn_Green" 0.0))
      (:`1`
        (`MeshComponent.SetScalarParameterValueOnMaterials` (`StaticMeshActor.StaticMeshComponent` (`self.PipeLight_2`)) "Turn_Green" 0.0))
      (:`2`
        (`MeshComponent.SetScalarParameterValueOnMaterials` (`StaticMeshActor.StaticMeshComponent` (`self.PipeLight_3`)) "Turn_Green" 0.0))
      (:`3`
        (`MeshComponent.SetScalarParameterValueOnMaterials` (`StaticMeshActor.StaticMeshComponent` (`self.PipeLight_4`)) "Turn_Green" 0.0)))))

(event `Multicast_ClientReleaseLeftHandScanner`
  (if (not (`KismetSystemLibrary.IsDedicatedServer`))
    (`MeshComponent.SetScalarParameterValueOnMaterials` (`/Game/Bo/Scripts/Handscanners/BP_Base_Handscanner.Stuff_02_V01_low_Scanner_low` (`self.HandScanner_L`)) "Emissive_Switch" 1.0)))

(event `Multicast_ClientPressRightHandScanner`
  (if (not (`KismetSystemLibrary.IsDedicatedServer`))
    (`MeshComponent.SetScalarParameterValueOnMaterials` (`/Game/Bo/Scripts/Handscanners/BP_Base_Handscanner.Stuff_02_V01_low_Scanner_low` (`self.HandScanner_R`)) "Emissive_Switch" 10.0)))

(event `Multicast_ClientReleaseRightHandScanner`
  (if (not (`KismetSystemLibrary.IsDedicatedServer`))
    (`MeshComponent.SetScalarParameterValueOnMaterials` (`/Game/Bo/Scripts/Handscanners/BP_Base_Handscanner.Stuff_02_V01_low_Scanner_low` (`self.HandScanner_R`)) "Emissive_Switch" 1.0)))

(event `Multicast_TurnOnPillars`
  (bind _pillers (`self.Pillers`))
  (bind _returnvalue (+ (`KismetArrayLibrary.Array_Length` _pillers) 1))
  (`KismetSystemLibrary.Delay` 0.1)
  (if (not (`KismetSystemLibrary.IsDedicatedServer`))
    (bind _counter (`/Game/EditorBlueprintResources/StandardMacros.Do N` _returnvalue :!label _label_5)
      (:`Exit`
        (if (== _counter _returnvalue)
          (`MeshComponent.SetScalarParameterValueOnMaterials` (`StaticMeshActor.StaticMeshComponent` (`self.HeroPiller`)) "Emissive_Intensity" 150.0)
          (else
            (`MeshComponent.SetScalarParameterValueOnMaterials` (`StaticMeshActor.StaticMeshComponent` (`|GetArrayItem` _pillers (- _counter 1))) "Emissive_Intensity" 75.0)
            (`KismetSystemLibrary.Delay` 0.5)
            (goto _label_5)))))))

(fn `AreAllKnobsCorrect`
  (params (KnobValues :type "Array of Boolean"))
  (returns (AllKnobsCorrect :type Boolean))
  (for _array_element KnobValues
    (if (not _array_element)
      (return false)))
  (return true))

(fn `AreAllValvesCorrect`
  (params (ValveValues :type "Array of Boolean"))
  (returns (AllValvesCorrect :type Boolean))
  (for _array_element ValveValues
    (if (not _array_element)
      (return false)))
  (return true))

(fn `UserConstructionScript`)