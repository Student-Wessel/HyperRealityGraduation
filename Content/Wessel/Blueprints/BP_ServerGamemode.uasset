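; BP_ServerGamemode is a game mode that hands pre-placed pawns to joining players on a dedicated server.
; HandleStartingNewPlayer waits briefly, increments CurrentPlayer and has the first two players possess Pawn1 and Pawn2, with debug prints.
; BeginPlay gathers OnlineTrackedPawn actors after a delay, but its loop body is empty.
; The display-name matching that assigns Pawn1 and Pawn2 is disconnected, so this graph never sets either variable.
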(event `self.ReceiveBeginPlay`
  (`KismetSystemLibrary.Delay` 1.0)
  (bind _outactors (`GameplayStatics.GetAllActorsOfClass` "/Game/OculusRetargeting/UnrealManequin/OnlineTrackedPawn.OnlineTrackedPawn_C"))
  (for _array_element _outactors
    _))

(event `self.HandleStartingNewPlayer`
  (params (NewPlayer :type "PlayerController Object Reference"))
  (`KismetSystemLibrary.PrintString` "player joined")
  (`KismetSystemLibrary.Delay` 2.0)
  (if (`KismetSystemLibrary.IsDedicatedServer`)
    (bind _result (`/Engine/EditorBlueprintResources/StandardMacros.IncrementInt` (`self.CurrentPlayer`))
      (:`  `
        (switch `int` _result
          (:`1`
            (`Controller.Possess` NewPlayer (`self.Pawn1`))
            (`KismetSystemLibrary.PrintString` "Posses pawn 1"))
          (:`2`
            (`Controller.Possess` NewPlayer (`self.Pawn2`))
            (`KismetSystemLibrary.PrintString` "Posses pawn 2")))))))

(fn `UserConstructionScript`)