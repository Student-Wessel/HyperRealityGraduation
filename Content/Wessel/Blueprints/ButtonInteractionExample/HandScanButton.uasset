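; Hand-scan button that fires pressed and released events based on how close the player's hands are.
; Each tick it gets both hand components from player pawn 0 through a message call and measures their distance to the Box component.
; It presses when either hand comes within about 25 units and releases once both move away, with an IsPressed flag preventing repeat calls.
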(event `self.ReceiveTick`
  (params (DeltaSeconds :type "Float (single-precision)"))
  (bind _returnvalue (`SceneComponent.K2_GetComponentLocation` (`self.Box`)))
  (bind (_lefthand _righthand) (message `/Game/Wessel/Blueprints/ButtonInteractionExample/PlayerHandTransform.GetPlayerHands` (`GameplayStatics.GetPlayerPawn` 0)))
  (if (`self.IsPressed`)
    (bind _returnvalue_2 (`KismetMathLibrary.VSize` (- (.location _lefthand) _returnvalue)))
    (bind _returnvalue_3 (`KismetMathLibrary.VSize` (- _returnvalue (.location _righthand))))
    (if (and (> _returnvalue_2 24.9) (> _returnvalue_3 24.9))
      (`self.ButtonReleased`)
      (set `self.IsPressed` false))
    (elif (or (< _returnvalue_2 25.0) (< _returnvalue_3 25.0))
      (`self.ButtonPressed`)
      (set `self.IsPressed` true))))

(fn `GetPlayerHands`
  (returns (LeftHand :type "Transform Structure") (RightHand :type "Transform Structure"))
  (return))

(fn `UserConstructionScript`)