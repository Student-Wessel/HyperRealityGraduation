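; ConsolTest is an example two-button puzzle actor that fires a one-time start event when both hand buttons are held at once.
; On BeginPlay, only on a dedicated server, it binds press and release events from its Lefthand and Righthand buttons.
; Both share a held-button counter; when it exceeds one, every actor implementing BPI_StartInteraction receives InteractionMessage, guarded by a done flag.
; Debug strings print each step.
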(event `self.ReceiveBeginPlay`
  (bind _lefthand (`self.Lefthand`))
  (bind _righthand (`self.Righthand`))
  (if (`KismetSystemLibrary.IsDedicatedServer`)
    (`|ExecutionSequence`
      (:`then_0`
        (`KismetSystemLibrary.PrintString` "Set bind 1")
        (add `/Game/Bo/Scripts/Handscanners/BP_Base_Handscanner.ButtonPress` _lefthand (delegate `Button1Pressed_Event`))
        (add `/Game/Bo/Scripts/Handscanners/BP_Base_Handscanner.ButtonRelease` _lefthand (delegate `Button1Released_Event`)))
      (:`then_1`
        (`KismetSystemLibrary.PrintString` "Set bind 2")
        (add `/Game/Bo/Scripts/Handscanners/BP_Base_Handscanner.ButtonPress` _righthand (delegate `Button2Pressed_Event`))
        (add `/Game/Bo/Scripts/Handscanners/BP_Base_Handscanner.ButtonRelease` _righthand (delegate `Button2Released_Event`))))))

(event `Button1Pressed_Event`
  (`KismetSystemLibrary.PrintString` "Button ++" :!label _label)
  (bind _result (`/Engine/EditorBlueprintResources/StandardMacros.IncrementInt` (`self.ButtonPressedAmount`))
    (:`  `
      (`KismetSystemLibrary.PrintString` (`KismetStringLibrary.Conv_IntToString` _result))
      (if (> (`self.ButtonPressedAmount`) 1)
        (`KismetSystemLibrary.PrintString` "First puzzle done" true true (struct :`R` 1.0 :`B` 0.018721 :`A` 1.0))
        (if (not (`self.StartEventsDone`))
          (set `self.StartEventsDone` true)
          (bind _outactors (`GameplayStatics.GetAllActorsWithInterface` "/Game/Bo/Scripts/BPI_StartInteraction.BPI_StartInteraction_C"))
          (for _array_element _outactors
            (message `/Game/Bo/Scripts/BPI_StartInteraction.Interaction` _array_element)))))))

(event `Button1Released_Event`
  (`/Engine/EditorBlueprintResources/StandardMacros.DecrementInt` (`self.ButtonPressedAmount`) :!label _label_2))

(event `Button2Pressed_Event`
  (goto _label))

(event `Button2Released_Event`
  (goto _label_2))

(fn `UserConstructionScript`)