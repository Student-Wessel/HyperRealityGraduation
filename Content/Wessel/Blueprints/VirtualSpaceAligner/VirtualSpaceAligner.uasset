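; VirtualSpaceAligner fits tagged virtual anchor actors to the player's physical Quest room.
; It loads the MRUK scene and retries until the room has four walls, floor and ceiling.
; Walls are sorted using player position and room center, and an opposite pair sets the room's heading.
; North/East/South/West, floor and ceiling anchors move there with offsets, then OnlineTrackedPawns receive the room-center transform.
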(event `AlignCurrentVirtualSpace`
  (bind _returnvalue (`AndroidPermissionFunctionLibrary.CheckPermission` "com.oculus.permission.USE_SCENE"))
  (if (not _returnvalue)
    (`KismetSystemLibrary.PrintString` "No permission" true true (struct :`R` 1.0 :`B` 0.006241 :`A` 1.0) 5.0)
    (`AndroidPermissionFunctionLibrary.AcquirePermissions` (`|MakeArray` "com.oculus.permission.USE_SCENE")))
  (`KismetSystemLibrary.PrintString` "Starting to Load" true true (struct :`R` 1.0 :`G` 0.90682 :`A` 1.0))
  (`MRUKSubsystem.LoadSceneFromDevice` (subsystem `MRUKSubsystem`) 256)
  (`KismetSystemLibrary.PrintString` "Loaded from device")
  (if (`KismetSystemLibrary.IsValid` (`self.OculusXRSceneActor`))
    (`KismetSystemLibrary.Delay` 0.25)
    (`OculusXRSceneActor.PopulateScene` (`self.OculusXRSceneActor`))
    (`self.WaitTillPopulated`)
    (else
      (`KismetSystemLibrary.PrintString` "Oculus XRScene Actor not assigned"))))

(event `WaitTillPopulated`
  (bind _walls_sorted (`self.Walls Sorted`))
  (bind _returnvalue (`MRUKSubsystem.GetCurrentRoom` (subsystem `MRUKSubsystem`)))
  (bind _output (`|GetArrayItem` _walls_sorted 2))
  (bind _output_2 (`|GetArrayItem` _walls_sorted))
  (bind _z (.z (`self.K2_GetActorLocation` (`MRUKRoom.FloorAnchor` (`MRUKSubsystem.GetCurrentRoom` (subsystem `MRUKSubsystem`))))))
  (if (`KismetSystemLibrary.IsValid` _returnvalue)
    (if (== (`KismetArrayLibrary.Array_Length` (`MRUKRoom.WallAnchors` _returnvalue)) 4)
      (if (`KismetSystemLibrary.IsValid` (`MRUKRoom.CeilingAnchor` _returnvalue))
        (if (`KismetSystemLibrary.IsValid` (`MRUKRoom.FloorAnchor` _returnvalue))
          (`KismetSystemLibrary.PrintString` "Scene is populated")
          (`KismetArrayLibrary.Array_Clear` (`self.Walls Sorted`))
          (`KismetArrayLibrary.Array_Clear` (`self.Walls Unsorted`))
          (set `self.Room Center` (`KismetMathLibrary.MakeVector` (.x (`self.K2_GetActorLocation` (`MRUKRoom.FloorAnchor` (`MRUKSubsystem.GetCurrentRoom` (subsystem `MRUKSubsystem`))))) (.y (`self.K2_GetActorLocation` (`MRUKRoom.FloorAnchor` (`MRUKSubsystem.GetCurrentRoom` (subsystem `MRUKSubsystem`))))) _z))
          (set `self.GroundZ` _z)
          (set `self.PlayerStartPosition` (`self.K2_GetActorLocation` (`Controller.K2_GetPawn` (`GameplayStatics.GetPlayerController` 0))))
          (for _array_element (`MRUKRoom.WallAnchors` (`MRUKSubsystem.GetCurrentRoom` (subsystem `MRUKSubsystem`)))
            (`KismetArrayLibrary.Array_Add` (`self.Walls Unsorted`) (`self.GetTransform` _array_element)))
          (`|ExecutionSequence`
            (:`then_0`
              (bind _returnvalue_2 (`HyperRealityRoomUtils.SortWalls` (`self.Walls Unsorted`) (`self.PlayerStartPosition`) (`self.Room Center`)))
              (set `self.Walls Sorted` _returnvalue_2))
            (:`then_1`
              (bind _output_get (set `self.Floor` (`self.GetTransform` (`MRUKRoom.FloorAnchor` (`MRUKSubsystem.GetCurrentRoom` (subsystem `MRUKSubsystem`))))))
              (set `self.Ceiling` (`self.GetTransform` (`MRUKRoom.CeilingAnchor` (`MRUKSubsystem.GetCurrentRoom` (subsystem `MRUKSubsystem`)))))
              (`|SpawnActorFromClass` "/Game/Wessel/Blueprints/TestCenterPoint.TestCenterPoint_C" _output "AlwaysSpawn" "MultiplyWithRoot" null null)
              (`|SpawnActorFromClass` "/Game/Wessel/Blueprints/TestCenterPoint.TestCenterPoint_C" _output_2 "AlwaysSpawn" "MultiplyWithRoot" null null)
              (bind _output_get_2 (set `self.RoomNormal` (`KismetMathLibrary.Normal` (- (.location _output) (.location _output_2)))))
              (bind _output_get_3 (set `self.PhysicalCenterPoint` (`KismetMathLibrary.MakeVector` (.x (.location _output_get)) (.y (.location _output_get)) (.z (.location _output_get)))))
              (bind _output_get_4 (set `self.PhysicalRoomNormal` (`KismetMathLibrary.MakeRotFromX` _output_get_2)))
              (`|SpawnActorFromClass` "/Game/Wessel/Blueprints/TestCenterPoint.TestCenterPoint_C" (`KismetMathLibrary.MakeTransform` _output_get_3 _output_get_4) "AlwaysSpawn" "MultiplyWithRoot" null null)
              (`OculusXRSceneActor.ClearScene` (`self.OculusXRSceneActor`))
              (`|ExecutionSequence`
                (:`then_0`
                  (bind _outactors (`GameplayStatics.GetAllActorsWithTag` "NorthAnchor"))
                  (for _array_element_2 _outactors
                    (`KismetArrayLibrary.Array_AddUnique` (`self.NorthWallAnchor`) _array_element_2)))
                (:`then_1`
                  (bind _outactors_2 (`GameplayStatics.GetAllActorsWithTag` "EastAnchor"))
                  (for _array_element_3 _outactors_2
                    (`KismetArrayLibrary.Array_AddUnique` (`self.EastWallAnchor`) _array_element_3)))
                (:`then_2`
                  (bind _outactors_3 (`GameplayStatics.GetAllActorsWithTag` "SouthAnchor"))
                  (for _array_element_4 _outactors_3
                    (`KismetArrayLibrary.Array_AddUnique` (`self.SouthWallAnchor`) _array_element_4)))
                (:`then_3`
                  (bind _outactors_4 (`GameplayStatics.GetAllActorsWithTag` "WestAnchor"))
                  (for _array_element_5 _outactors_4
                    (`KismetArrayLibrary.Array_AddUnique` (`self.WestWallAnchor`) _array_element_5)))
                (:`then_4`
                  (bind _outactors_5 (`GameplayStatics.GetAllActorsWithTag` "FloorAnchor"))
                  (for _array_element_6 _outactors_5
                    (`KismetArrayLibrary.Array_AddUnique` (`self.FloorActorAnchor`) _array_element_6)))
                (:`then_5`
                  (bind _outactors_6 (`GameplayStatics.GetAllActorsWithTag` "CeilingAnchor"))
                  (for _array_element_7 _outactors_6
                    (`KismetArrayLibrary.Array_AddUnique` (`self.CeilingActorAnchor`) _array_element_7)))
                (:`then_6`
                  (`KismetSystemLibrary.PrintString` "Set geometry")
                  (`|ExecutionSequence`
                    (:`then_0`
                      (for _array_element_8 (`self.NorthWallAnchor`)
                        (if (`KismetSystemLibrary.IsValid` _array_element_8)
                          (`self.K2_SetActorTransform` _array_element_8 (`KismetMathLibrary.MakeTransform` (`KismetMathLibrary.MakeVector` (.x (.location (`|GetArrayItem` (`self.Walls Sorted`)))) (.y (.location (`|GetArrayItem` (`self.Walls Sorted`)))) (`self.GroundZ`)) (`KismetMathLibrary.MakeRotFromX` (`self.RoomNormal`)) (.scale (`|GetArrayItem` (`self.Walls Sorted`)))) false true)
                          (`self.K2_AddActorWorldRotation` :`self` _array_element_8)
                          (`self.K2_AddActorLocalTransform` _array_element_8 (`self.NorthWallOffset`) false true))))
                    (:`then_1`
                      (for _array_element_9 (`self.EastWallAnchor`)
                        (if (`KismetSystemLibrary.IsValid` _array_element_9)
                          (`self.K2_SetActorTransform` _array_element_9 (`KismetMathLibrary.MakeTransform` (`KismetMathLibrary.MakeVector` (.x (.location (`|GetArrayItem` (`self.Walls Sorted`) 1))) (.y (.location (`|GetArrayItem` (`self.Walls Sorted`) 1))) (`self.GroundZ`)) (`KismetMathLibrary.MakeRotFromX` (`self.RoomNormal`)) (.scale (`|GetArrayItem` (`self.Walls Sorted`) 1))) false true)
                          (`self.K2_AddActorWorldRotation` :`self` _array_element_9)
                          (`self.K2_AddActorLocalTransform` _array_element_9 (`self.EastWallOffset`) false true))))
                    (:`then_2`
                      (for _array_element_10 (`self.SouthWallAnchor`)
                        (if (`KismetSystemLibrary.IsValid` _array_element_10)
                          (`self.K2_SetActorTransform` _array_element_10 (`KismetMathLibrary.MakeTransform` (`KismetMathLibrary.MakeVector` (.x (.location (`|GetArrayItem` (`self.Walls Sorted`) 2))) (.y (.location (`|GetArrayItem` (`self.Walls Sorted`) 2))) (`self.GroundZ`)) (`KismetMathLibrary.MakeRotFromX` (`self.RoomNormal`)) (.scale (`|GetArrayItem` (`self.Walls Sorted`) 2))) false true)
                          (`self.K2_AddActorWorldRotation` :`self` _array_element_10)
                          (`self.K2_AddActorLocalTransform` _array_element_10 (`self.SouthWallOffset`) false true))))
                    (:`then_3`
                      (for _array_element_11 (`self.WestWallAnchor`)
                        (if (`KismetSystemLibrary.IsValid` _array_element_11)
                          (`self.K2_SetActorTransform` _array_element_11 (`KismetMathLibrary.MakeTransform` (`KismetMathLibrary.MakeVector` (.x (.location (`|GetArrayItem` (`self.Walls Sorted`) 3))) (.y (.location (`|GetArrayItem` (`self.Walls Sorted`) 3))) (`self.GroundZ`)) (`KismetMathLibrary.MakeRotFromX` (`self.RoomNormal`)) (.scale (`|GetArrayItem` (`self.Walls Sorted`) 3))) false true)
                          (`self.K2_AddActorWorldRotation` :`self` _array_element_11)
                          (`self.K2_AddActorLocalTransform` _array_element_11 (`self.WestWallOffset`) false true))))
                    (:`then_4`
                      (for _array_element_12 (`self.FloorActorAnchor`)
                        (if (`KismetSystemLibrary.IsValid` _array_element_12)
                          (`self.K2_SetActorTransform` _array_element_12 (`KismetMathLibrary.MakeTransform` (`KismetMathLibrary.MakeVector` (.x (.location (`self.Floor`))) (.y (.location (`self.Floor`))) (`self.GroundZ`)) (`KismetMathLibrary.MakeRotFromX` (`self.RoomNormal`)) (.scale (`self.Floor`))) false true)
                          (`self.K2_AddActorLocalRotation` :`self` _array_element_12)
                          (`self.K2_AddActorLocalTransform` _array_element_12 (`self.FloorOffset`) false true))))
                    (:`then_5`
                      (for _array_element_13 (`self.CeilingActorAnchor`)
                        (if (`KismetSystemLibrary.IsValid` _array_element_13)
                          (`self.K2_SetActorTransform` _array_element_13 (`KismetMathLibrary.MakeTransform` (`KismetMathLibrary.MakeVector` (.x (.location (`self.Ceiling`))) (.y (.location (`self.Ceiling`))) (+ (`self.Ceiling_Height`) (`self.GroundZ`))) (`KismetMathLibrary.MakeRotFromX` (`self.RoomNormal`)) (.scale (`self.Ceiling`))) false true)
                          (`self.K2_AddActorLocalRotation` :`self` _array_element_13)
                          (`self.K2_AddActorLocalTransform` _array_element_13 (`self.CeilingOffset`) false true))))))
                (:`then_7`
                  (bind _asonline_tracked_pawn (cast `/Game/OculusRetargeting/UnrealManequin/OnlineTrackedPawn` (`Controller.K2_GetPawn` (`GameplayStatics.GetPlayerController` 0)))
                    (:`then`
                      (bind _output_get_5 (set `/Game/OculusRetargeting/UnrealManequin/OnlineTrackedPawn.RoomCenterTransfrom` (`KismetMathLibrary.MakeTransform` (`self.PhysicalCenterPoint`) (`self.PhysicalRoomNormal`)) _asonline_tracked_pawn))
                      (bind _outactors_7 (`GameplayStatics.GetAllActorsOfClass` "/Game/OculusRetargeting/UnrealManequin/OnlineTrackedPawn.OnlineTrackedPawn_C"))
                      (for _array_element_14 _outactors_7
                        (if (!= _array_element_14 self)
                          (`/Game/OculusRetargeting/UnrealManequin/OnlineTrackedPawn.RoomCalibratedCallback` _array_element_14 _output_get_5))))
                    (:`CastFailed`
                      (`KismetSystemLibrary.PrintString` "Got worng player actor type when trying to set offset")))))))
          (else
            (`KismetSystemLibrary.PrintString` "No Floor anchor")
            (`KismetSystemLibrary.Delay` 1.0 :!label _label)
            (`KismetSystemLibrary.PrintString` "Room not ready")
            (`self.WaitTillPopulated`)))
        (else
          (`KismetSystemLibrary.PrintString` "No Ceiling anchor")
          (goto _label)))
      (else
        (`KismetSystemLibrary.PrintString` "Wall count not correct")
        (goto _label)))
    (else
      (goto _label))))

(fn `UserConstructionScript`)