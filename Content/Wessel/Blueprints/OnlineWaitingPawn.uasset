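; Pawn for the online waiting stage that hands each player off to a transition by fading to black.
; A client request event finds the BP_FadeToBlack actor, binds to its sequence player's finish event and plays it.
; When the fade ends, the pawn destroys Oculus XR persistent passthrough and notifies the server.
; The server event then tells OnlineWaitingGamemode that it is ready to transition.
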(event `Client_RequestTurnToBlack`
  (`KismetSystemLibrary.PrintString` "Request to fade black")
  (bind _returnvalue (`GameplayStatics.GetActorOfClass` "/Game/Wessel/LevelSeqences/BP_FadeToBlack.BP_FadeToBlack_C"))
  (if (`KismetSystemLibrary.IsValid` _returnvalue)
    (bind _sequenceplayer (`LevelSequenceActor.SequencePlayer` _returnvalue))
    (add `MovieSceneSequencePlayer.OnFinished` _sequenceplayer (delegate `FadedToBlack`))
    (`MovieSceneSequencePlayer.Play` _sequenceplayer)
    (else
      (`KismetSystemLibrary.PrintString` "No fade blueprint found"))))

(event `FadedToBlack`
  (`OculusXRPassthroughSubsystem.DestroyPersistentPassthrough` (subsystem `OculusXRPassthroughSubsystem`))
  (`self.Server_NotifyServerReady`)
  (`KismetSystemLibrary.PrintString` "Notify server"))

(event `Server_NotifyServerReady`
  (bind _returnvalue (`GameplayStatics.GetGameMode`))
  (if (`KismetSystemLibrary.IsValid` _returnvalue)
    (bind _asonline_waiting_gamemode (cast `/Game/Wessel/Blueprints/OnlineWaitingGamemode` _returnvalue)
      (:`then`
        (`/Game/Wessel/Blueprints/OnlineWaitingGamemode.NotifyReadyToTransition` _asonline_waiting_gamemode))
      (:`CastFailed`
        (`KismetSystemLibrary.PrintString` "Gamemode was not waiting online gamemode")))
    (else
      (`KismetSystemLibrary.PrintString` "Gamemode not falid"))))

(fn `UserConstructionScript`)