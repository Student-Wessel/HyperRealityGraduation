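; SimpleCubePawn is a pawn that exercises variable replication.
; Each tick it passes its time since creation to the SendToServer event, which writes it into NetworkedVariable.
; The variable's OnRep function prints the new value, while an unconnected debug print of the pawn's name and local and remote roles never runs.
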(event `self.ReceiveBeginPlay`)

(event `self.ReceiveTick`
  (params (DeltaSeconds :type "Float (single-precision)"))
  (`self.SendToServer` (`self.GetGameTimeSinceCreation`)))

(event `SendToServer`
  (params (Data :type "Float (double-precision)"))
  (set `self.NetworkedVariable` Data))

(fn `OnRep_NetworkedVariable`
  (`KismetSystemLibrary.PrintString` (`KismetStringLibrary.Conv_DoubleToString` (`self.NetworkedVariable`))))

(fn `UserConstructionScript`)