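; Game mode for an online waiting room that gathers players on a dedicated server before the match.
; On login it records each player, and once two have joined it waits briefly and asks each player's OnlineWaitingPawn to fade to black.
; A ready notification counts players who finished transitioning, and when two are ready it opens MasterLevelV2 after a short delay.
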(event `self.K2_PostLogin`
  (params (NewPlayer :type "PlayerController Object Reference"))
  (if (`KismetSystemLibrary.IsDedicatedServer`)
    (`KismetArrayLibrary.Array_AddUnique` (`self.PlayersInWaitingRoom`) NewPlayer)
    (bind _result (`/Engine/EditorBlueprintResources/StandardMacros.IncrementInt` (`self.PlayerCount`))
      (:`  `
        (if (>= _result 2)
          (`KismetSystemLibrary.Delay` 2.0)
          (bind _array_element (`/Game/EditorBlueprintResources/StandardMacros.ForEachLoop` (`self.PlayersInWaitingRoom`))
            (:`LoopBody`
              (bind _asonline_waiting_pawn (cast `/Game/Wessel/Blueprints/OnlineWaitingPawn` (`Controller.K2_GetPawn` _array_element))
                (:`then`
                  (`/Game/Wessel/Blueprints/OnlineWaitingPawn.Client_RequestTurnToBlack` _asonline_waiting_pawn)
                  (`KismetSystemLibrary.PrintString` "Send request to player to fade to black"))
                (:`CastFailed`
                  (`KismetSystemLibrary.PrintString` "######################## Wrong pawn, not a online waiting player ##################################"))))))))))

(event `NotifyReadyToTransition`
  (`KismetSystemLibrary.PrintString` "Player has gone ready")
  (bind _result (`/Game/EditorBlueprintResources/StandardMacros.IncrementInt` (`self.PlayerReadyCount`))
    (:`  `
      (if (>= _result 2)
        (`KismetSystemLibrary.Delay` 1.0)
        (`GameplayStatics.OpenLevelBySoftObjectPtr` "/Game/Wessel/Map/MasterLevelV2.MasterLevelV2")))))

(fn `UserConstructionScript`)