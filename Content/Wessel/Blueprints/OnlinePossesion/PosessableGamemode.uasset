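; Game mode that assigns joining players to pre-placed PosessablePawn actors in an online possession setup.
; One second after BeginPlay it finds those pawns and caches Pawn1 and Pawn2 by matching display names.
; On a dedicated server only, HandleStartingNewPlayer increments a player count and switches on it to possess either cached pawn, with debug prints.
; Possession does not wait for the delayed pawn lookup to finish.
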(event `self.ReceiveBeginPlay`
  (`KismetSystemLibrary.Delay` 1.0)
  (bind _outactors (`GameplayStatics.GetAllActorsOfClass` "/Game/Wessel/Blueprints/OnlinePossesion/PosessablePawn.PosessablePawn_C"))
  (for _array_element _outactors
    (bind _returnvalue (`KismetSystemLibrary.GetDisplayName` _array_element))
    (if (`KismetStringLibrary.EqualEqual_StrStr` _returnvalue "Pawn1")
      (set `self.Pawn1` _array_element)
      (elif (`KismetStringLibrary.EqualEqual_StrStr` _returnvalue "Pawn2")
        (set `self.Pawn2` _array_element)))))

(event `self.HandleStartingNewPlayer`
  (params (NewPlayer :type "PlayerController Object Reference"))
  (if (`KismetSystemLibrary.IsDedicatedServer`)
    (bind _result (`/Engine/EditorBlueprintResources/StandardMacros.IncrementInt` (`self.CurrentPlayerCount`))
      (:`  `
        (switch `int` _result
          (:`1`
            (`Controller.Possess` NewPlayer (`self.Pawn1`))
            (`KismetSystemLibrary.PrintString` "Posses pawn 1")
            (`KismetSystemLibrary.Delay` 0.5))
          (:`2`
            (`Controller.Possess` NewPlayer (`self.Pawn2`))
            (`KismetSystemLibrary.PrintString` "Posses pawn 2")
            (`KismetSystemLibrary.Delay` 0.5)))))))

(fn `UserConstructionScript`)