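; Tracks the sea monster's health and relays its death and attack pattern to clients.
; DealDamage subtracts health and, once it reaches zero, multicasts a single death notice.
; The first hit also generates a random attack sequence and multicasts it once.
; Non-dedicated instances handle the multicasts by lazily finding and caching BP_SeaMonster, then triggering its death or setting its pattern.
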(event `DealDamage`
  (params (Damage :type Integer))
  (`|ExecutionSequence`
    (:`then_0`
      (bind _output_get (set `self.Health` (- (`self.Health`) Damage)))
      (`KismetSystemLibrary.PrintString` (`KismetStringLibrary.BuildString_Int` "" "Damage dealth, new health: " _output_get))
      (if (<= _output_get 0)
        (set `self.Health` 0)
        (if (not (`self.IsDead`))
          (`self.Multicast_SeaMonsterDeadNotify`)
          (set `self.IsDead` true))))
    (:`then_1`
      (if (not (`self.AttackPatternSend`))
        (`KismetArrayLibrary.Array_Clear` (`self.AttackPattern`))
        (for _ (range 15)
          (`KismetArrayLibrary.Array_Add` (`self.AttackPattern`) (`KismetMathLibrary.RandomInteger` 3)))
        (`self.Multicast_SendAttackPatternToClient` (`self.AttackPattern`))
        (set `self.AttackPatternSend` true)))))

(event `Multicast_SeaMonsterDeadNotify`
  (if (`KismetSystemLibrary.IsDedicatedServer`)
    _
    (elif (`self.SeaMonsterSet`)
      (`/Game/Liam/Ani/Monster/BP_SeaMonster.LetMonsterDie` (`self.SeaMonster`) :!label _label)
      (else
        (bind _returnvalue (`GameplayStatics.GetActorOfClass` "/Game/Liam/Ani/Monster/BP_SeaMonster.BP_SeaMonster_C"))
        (if (`KismetSystemLibrary.IsValid` _returnvalue)
          (set `self.SeaMonster` _returnvalue)
          (set `self.SeaMonsterSet` true)
          (goto _label))))))

(event `Multicast_SendAttackPatternToClient`
  (params (AttackPattern :type "Array of Integer"))
  (if (`KismetSystemLibrary.IsDedicatedServer`)
    _
    (elif (`self.SeaMonsterSet`)
      (`/Game/Liam/Ani/Monster/BP_SeaMonster.SetAttackPattern` (`self.SeaMonster`) AttackPattern :!label _label_2)
      (else
        (bind _returnvalue (`GameplayStatics.GetActorOfClass` "/Game/Liam/Ani/Monster/BP_SeaMonster.BP_SeaMonster_C"))
        (if (`KismetSystemLibrary.IsValid` _returnvalue)
          (set `self.SeaMonster` _returnvalue)
          (set `self.SeaMonsterSet` true)
          (goto _label_2))))))

(fn `UserConstructionScript`)