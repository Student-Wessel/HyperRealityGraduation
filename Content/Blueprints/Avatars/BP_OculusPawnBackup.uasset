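; Backup Oculus VR pawn whose BeginPlay only calls its parent; its own setup, update and click logic is disconnected.
; The unused functions aim widget interaction pointers from hand-tracking poses or motion controllers, placing cursor spheres on focusable widget hits.
; They also hide low-confidence hands' cursors and toggle controller visibility.
; Other orphaned chains tint cursors on press and release, and set a delayed floor tracking origin to avoid a floor-stuck avatar.
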(event `self.ReceiveBeginPlay`
  (`parent.ReceiveBeginPlay`))

(event `self.ReceiveTick`
  (params (DeltaSeconds :type "Float (single-precision)")))

(fn `UpdateControllers`
  (`SceneComponent.SetVisibility` (`self.MotionControllerLeft`) (and (not (`OculusXRInputFunctionLibrary.IsHandTrackingEnabled`)) (`self.DisplayControllers`)) true)
  (`SceneComponent.SetVisibility` (`self.MotionControllerRight`) (and (not (`OculusXRInputFunctionLibrary.IsHandTrackingEnabled`)) (`self.DisplayControllers`)) true))

(fn `UpdateWidgetInteractions`
  (bind (_returnvalue_location _returnvalue_rotation) (`KismetMathLibrary.BreakTransform` (`OculusXRInputFunctionLibrary.GetPointerPose` "HandLeft")))
  (bind (_returnvalue_location_2 _returnvalue_rotation_2) (`KismetMathLibrary.BreakTransform` (`OculusXRInputFunctionLibrary.GetPointerPose` "HandRight")))
  (bind _widgetinteractionright (`self.WidgetInteractionRight`))
  (bind _widgetinteractionleft (`self.WidgetInteractionLeft`))
  (bind (_returnvalue_location_3 _returnvalue_rotation_3) (`KismetMathLibrary.BreakTransform` (`SceneComponent.GetRelativeTransform` (`self.MotionControllerRight`))))
  (bind (_returnvalue_location_4 _returnvalue_rotation_4) (`KismetMathLibrary.BreakTransform` (`SceneComponent.GetRelativeTransform` (`self.MotionControllerLeft`))))
  (bind (_bblockinghit _binitialoverlap _time _distance _location) (`GameplayStatics.BreakHitResult` (`WidgetInteractionComponent.GetLastHitResult` _widgetinteractionright)))
  (bind (_bblockinghit_2 _binitialoverlap_2 _time_2 _distance_2 _location_2) (`GameplayStatics.BreakHitResult` (`WidgetInteractionComponent.GetLastHitResult` _widgetinteractionleft)))
  (if (`OculusXRInputFunctionLibrary.IsHandTrackingEnabled`)
    (`|ExecutionSequence`
      (:`then_0`
        (switch `EOculusXRTrackingConfidence` (`OculusXRInputFunctionLibrary.GetTrackingConfidence` "HandLeft")
          (:`Low`
            (`SceneComponent.SetVisibility` (`self.InteractionSphereLeft`) false false :!label _label))
          (:`High`
            (if (`OculusXRInputFunctionLibrary.IsPointerPoseValid` "HandLeft")
              (`SceneComponent.K2_SetRelativeLocationAndRotation` (`self.WidgetInteractionLeft`) _returnvalue_location _returnvalue_rotation false false)
              (`SceneComponent.SetVisibility` (`self.InteractionSphereLeft`) (`WidgetInteractionComponent.IsOverFocusableWidget` _widgetinteractionleft) false :!label _label_2)
              (if _bblockinghit_2
                (`SceneComponent.K2_SetWorldLocation` (`self.InteractionSphereLeft`) _location_2 false false))
              (else
                (goto _label))))))
      (:`then_1`
        (switch `EOculusXRTrackingConfidence` (`OculusXRInputFunctionLibrary.GetTrackingConfidence` "HandRight")
          (:`Low`
            (`SceneComponent.SetVisibility` (`self.InteractionSphereRight`) false false :!label _label_3))
          (:`High`
            (if (`OculusXRInputFunctionLibrary.IsPointerPoseValid` "HandRight")
              (`SceneComponent.K2_SetRelativeLocationAndRotation` (`self.WidgetInteractionRight`) _returnvalue_location_2 _returnvalue_rotation_2 false false)
              (`SceneComponent.SetVisibility` (`self.InteractionSphereRight`) (`WidgetInteractionComponent.IsOverFocusableWidget` _widgetinteractionright) false :!label _label_4)
              (if _bblockinghit
                (`SceneComponent.K2_SetWorldLocation` (`self.InteractionSphereRight`) _location false false))
              (else
                (goto _label_3)))))))
    (else
      (`|ExecutionSequence`
        (:`then_0`
          (`SceneComponent.K2_SetRelativeLocationAndRotation` (`self.WidgetInteractionLeft`) _returnvalue_location_4 _returnvalue_rotation_4 false false)
          (goto _label_2))
        (:`then_1`
          (`SceneComponent.K2_SetRelativeLocationAndRotation` (`self.WidgetInteractionRight`) _returnvalue_location_3 _returnvalue_rotation_3 false false)
          (goto _label_4))))))

(fn `UserConstructionScript`)