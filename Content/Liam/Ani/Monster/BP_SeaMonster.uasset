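; Sea monster boss that runs its fight off dedicated servers: a timed intro, then repeated teleport, alert, rise, attack and dive cycles.
; Tick starts each delay-driven cycle via InLoop, using AttackPattern for position, though the index only advances on death.
; Bone-following head and body colliders destroy bullets and report damage to the local pawn.
; LetMonsterDie, also fired 30 seconds after BeginPlay, triggers a final surfacing, then quits the game.
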(event `self.ReceiveBeginPlay`
  (bind _monster_fightaudio (`self.Monster_FightAudio`))
  (bind _monster_fightaudio_2 (`self.Monster_FightAudio`))
  (bind _monster_fightaudio_3 (`self.Monster_FightAudio`))
  (bind _monster_fightaudio_4 (`self.Monster_FightAudio`))
  (bind _monster_fightaudio_5 (`self.Monster_FightAudio`))
  (bind _monster_fightaudio_6 (`self.Monster_FightAudio`))
  (if (not (`KismetSystemLibrary.IsDedicatedServer`))
    (`|ExecutionSequence`
      (:`then_0`
        (`KismetSystemLibrary.Delay` 1.0)
        (`AudioParameterControllerInterface.SetTriggerParameter` _monster_fightaudio_2 "tMonsterAlert")
        (`GameplayStatics.SpawnSoundAttached` "/Game/Liam/Audio/Monster/Monster_Audio.Monster_Audio" _monster_fightaudio_2 "None" (0.0 0.0 0.0) (struct) "KeepRelativeOffset" false 1.0 1.0 0.0 null null)
        (`KismetSystemLibrary.Delay` 2.0)
        (set `self.bStart` true)
        (set `self.fAlertMat_Opacity` 0.4)
        (`MeshComponent.SetScalarParameterValueOnMaterials` (`self.Monster_Alert1`) "Opacity" (`self.fAlertMat_Opacity`))
        (`AudioParameterControllerInterface.SetTriggerParameter` _monster_fightaudio "tWaterSplashUp")
        (`GameplayStatics.SpawnSoundAttached` "/Game/Liam/Audio/Monster/Monster_Audio.Monster_Audio" _monster_fightaudio "None" (0.0 0.0 0.0) (struct) "KeepRelativeOffset" false 1.0 1.0 0.0 null null)
        (`KismetSystemLibrary.Delay` 2.5)
        (`AudioParameterControllerInterface.SetTriggerParameter` _monster_fightaudio_6 "tWaterSplashDown")
        (`GameplayStatics.SpawnSoundAttached` "/Game/Liam/Audio/Monster/Monster_Audio.Monster_Audio" _monster_fightaudio_6 "None" (0.0 0.0 0.0) (struct) "KeepRelativeOffset" false 1.0 1.0 0.0 null null)
        (`KismetSystemLibrary.Delay` 1.0)
        (set `self.fAlertMat_Opacity` 0.0)
        (`MeshComponent.SetScalarParameterValueOnMaterials` (`self.Monster_Alert1`) "Opacity" (`self.fAlertMat_Opacity`))
        (`AudioParameterControllerInterface.SetTriggerParameter` _monster_fightaudio_3 "tMonsterEntrance")
        (`GameplayStatics.SpawnSoundAttached` "/Game/Liam/Audio/Monster/Monster_Audio.Monster_Audio" _monster_fightaudio_3 "None" (0.0 0.0 0.0) (struct) "KeepRelativeOffset" false 1.0 1.0 0.0 null null)
        (`KismetSystemLibrary.Delay` 7.0)
        (`KismetSystemLibrary.DelayUntilNextTick`)
        (set `self.bShouldJump` false)
        (set `self.bShouldGoDown` false)
        (set `self.bShouldAttack` true)
        (`AudioParameterControllerInterface.SetTriggerParameter` _monster_fightaudio_4 "tMonsterAttack")
        (`GameplayStatics.SpawnSoundAttached` "/Game/Liam/Audio/Monster/Monster_Audio.Monster_Audio" _monster_fightaudio_4 "None" (0.0 0.0 0.0) (struct) "KeepRelativeOffset" false 1.0 1.0 0.0 null null)
        (`KismetSystemLibrary.DelayUntilNextTick`)
        (set `self.bShouldAttack` false)
        (`KismetSystemLibrary.Delay` 8.0)
        (set `self.bShouldGoDown` true)
        (`AudioParameterControllerInterface.SetTriggerParameter` _monster_fightaudio_5 "tWaterSplashDown")
        (`GameplayStatics.SpawnSoundAttached` "/Game/Liam/Audio/Monster/Monster_Audio.Monster_Audio" _monster_fightaudio_5 "None" (0.0 0.0 0.0) (struct) "KeepRelativeOffset" false 1.0 1.0 0.0 null null)
        (set `self.inLoop` false))
      (:`then_1`
        (`KismetSystemLibrary.Delay` 1.0)
        (bind _asonline_tracked_pawn (cast `/Game/OculusRetargeting/UnrealManequin/OnlineTrackedPawn` (`Controller.K2_GetPawn` (`GameplayStatics.GetPlayerController` 0)))
          (:`then`
            (set `self.LocalPlayer` _asonline_tracked_pawn)
            (add `PrimitiveComponent.OnComponentBeginOverlap` (`self.BodyCollider`) (delegate `OnComponentBeginOverlapBody`))
            (add `PrimitiveComponent.OnComponentBeginOverlap` (`self.HeadCollider`) (delegate `OnComponentBeginOverlapHead`)))
          (:`CastFailed`
            (`KismetSystemLibrary.PrintString` "Not right player pawn"))))
      (:`then_2`
        (`KismetSystemLibrary.Delay` 30.0)
        (`self.LetMonsterDie`)))))

(event `OnComponentBeginOverlapBody`
  (params (OverlappedComponent :type "PrimitiveComponent Object Reference") (OtherActor :type "Actor Object Reference") (OtherComp :type "PrimitiveComponent Object Reference") (OtherBodyIndex :type Integer) (bFromSweep :type Boolean) (SweepResult :type "HitResult Structure (by ref)"))
  (if (not (`self.ShouldDie`))
    (bind _asbp_bullet (cast `/Game/Bo/Scripts/Gun/BP_Bullet` OtherActor))
    (if (`KismetSystemLibrary.IsValid` _asbp_bullet)
      (`self.K2_DestroyActor` _asbp_bullet)
      (`KismetSystemLibrary.PrintString` "Hit on body")
      (`/Game/OculusRetargeting/UnrealManequin/OnlineTrackedPawn.SeaMonsterDamage` (`self.LocalPlayer`) 1))))

(event `OnComponentBeginOverlapHead`
  (params (OverlappedComponent :type "PrimitiveComponent Object Reference") (OtherActor :type "Actor Object Reference") (OtherComp :type "PrimitiveComponent Object Reference") (OtherBodyIndex :type Integer) (bFromSweep :type Boolean) (SweepResult :type "HitResult Structure (by ref)"))
  (if (not (`self.ShouldDie`))
    (bind _asbp_bullet (cast `/Game/Bo/Scripts/Gun/BP_Bullet` OtherActor))
    (if (`KismetSystemLibrary.IsValid` _asbp_bullet)
      (`self.K2_DestroyActor` _asbp_bullet)
      (`KismetSystemLibrary.PrintString` "Hit on head")
      (`/Game/OculusRetargeting/UnrealManequin/OnlineTrackedPawn.SeaMonsterDamage` (`self.LocalPlayer`) 2))))

(event `self.ReceiveTick`
  (params (DeltaSeconds :type "Float (single-precision)"))
  (bind _skeletalmeshseamonster (`self.SkeletalMeshSeaMonster`))
  (bind _monster_fightaudio (`self.Monster_FightAudio`))
  (bind _monster_fightaudio_2 (`self.Monster_FightAudio`))
  (bind _monster_fightaudio_3 (`self.Monster_FightAudio`))
  (bind _monster_fightaudio_4 (`self.Monster_FightAudio`))
  (bind _monster_fightaudio_5 (`self.Monster_FightAudio`))
  (bind _monster_fightaudio_6 (`self.Monster_FightAudio`))
  (if (not (`KismetSystemLibrary.IsDedicatedServer`))
    (`|ExecutionSequence`
      (:`then_0`
        (if (`self.inLoop`)
          _
          (elif (== (`self.bIsDead`) false)
            (if (`self.ShouldDie`)
              (set `self.inLoop` true)
              (`KismetSystemLibrary.Delay` 1.0)
              (`self.K2_SetActorLocationAndRotation` (.location (`self.GetTransform` (`|GetArrayItem` (`self.bTeleportPositions`)))) (.rotation (`self.GetTransform` (`|GetArrayItem` (`self.bTeleportPositions`)))) false true)
              (bind _result (`/Engine/EditorBlueprintResources/StandardMacros.IncrementInt` (`self.AttackPatternIndex`))
                (:`  `
                  (if (> _result (`KismetArrayLibrary.Array_LastIndex` (`self.AttackPattern`)))
                    (set `self.AttackPatternIndex` 0))
                  (`AudioParameterControllerInterface.SetTriggerParameter` _monster_fightaudio_2 "tMonsterAlert")
                  (`GameplayStatics.SpawnSoundAttached` "/Game/Liam/Audio/Monster/Monster_Audio.Monster_Audio" _monster_fightaudio_2 "None" (0.0 0.0 0.0) (struct) "KeepRelativeOffset" false 1.0 1.0 0.0 null null)
                  (`KismetSystemLibrary.DelayUntilNextTick`)
                  (set `self.fAlertMat_Opacity` 0.4)
                  (`MeshComponent.SetScalarParameterValueOnMaterials` (`self.Monster_Alert1`) "Opacity" (`self.fAlertMat_Opacity`))
                  (`KismetSystemLibrary.Delay` 2.0)
                  (set `self.fAlertMat_Opacity` 0.0)
                  (`MeshComponent.SetScalarParameterValueOnMaterials` (`self.Monster_Alert1`) "Opacity" (`self.fAlertMat_Opacity`))
                  (set `self.bShouldGoDown` false)
                  (set `self.bShouldGoUp` true)
                  (`AudioParameterControllerInterface.SetTriggerParameter` _monster_fightaudio "tMonsterEntrance")
                  (`GameplayStatics.SpawnSoundAttached` "/Game/Liam/Audio/Monster/Monster_Audio.Monster_Audio" _monster_fightaudio "None" (0.0 0.0 0.0) (struct) "KeepRelativeOffset" false 1.0 1.0 0.0 null null)
                  (`KismetSystemLibrary.Delay` 2.0)
                  (set `self.bIsDead` true)
                  (`KismetSystemLibrary.Delay` 10.0)
                  (`KismetSystemLibrary.QuitGame` null "Quit")))
              (else
                (set `self.inLoop` true)
                (`KismetSystemLibrary.Delay` 1.0)
                (`self.K2_SetActorLocationAndRotation` (.location (`self.GetTransform` (`|GetArrayItem` (`self.bTeleportPositions`) (`|GetArrayItem` (`self.AttackPattern`) (`self.AttackPatternIndex`))))) (.rotation (`self.GetTransform` (`|GetArrayItem` (`self.bTeleportPositions`) (`|GetArrayItem` (`self.AttackPattern`) (`self.AttackPatternIndex`))))) false true)
                (`AudioParameterControllerInterface.SetTriggerParameter` _monster_fightaudio_3 "tMonsterAlert")
                (`GameplayStatics.SpawnSoundAttached` "/Game/Liam/Audio/Monster/Monster_Audio.Monster_Audio" _monster_fightaudio_3 "None" (0.0 0.0 0.0) (struct) "KeepRelativeOffset" false 1.0 1.0 0.0 null null)
                (`KismetSystemLibrary.DelayUntilNextTick`)
                (set `self.fAlertMat_Opacity` 0.4)
                (`MeshComponent.SetScalarParameterValueOnMaterials` (`self.Monster_Alert1`) "Opacity" (`self.fAlertMat_Opacity`))
                (`KismetSystemLibrary.Delay` 2.0)
                (set `self.fAlertMat_Opacity` 0.0)
                (`MeshComponent.SetScalarParameterValueOnMaterials` (`self.Monster_Alert1`) "Opacity" (`self.fAlertMat_Opacity`))
                (set `self.bShouldGoDown` false)
                (set `self.bShouldGoUp` true)
                (`AudioParameterControllerInterface.SetTriggerParameter` _monster_fightaudio_4 "tMonsterEntrance")
                (`GameplayStatics.SpawnSoundAttached` "/Game/Liam/Audio/Monster/Monster_Audio.Monster_Audio" _monster_fightaudio_4 "None" (0.0 0.0 0.0) (struct) "KeepRelativeOffset" false 1.0 1.0 0.0 null null)
                (`KismetSystemLibrary.Delay` 2.0)
                (set `self.bShouldAttack` true)
                (`AudioParameterControllerInterface.SetTriggerParameter` _monster_fightaudio_5 "tMonsterAttack")
                (`GameplayStatics.SpawnSoundAttached` "/Game/Liam/Audio/Monster/Monster_Audio.Monster_Audio" _monster_fightaudio_5 "None" (0.0 0.0 0.0) (struct) "KeepRelativeOffset" false 1.0 1.0 0.0 null null)
                (`KismetSystemLibrary.Delay` 2.0)
                (set `self.bShouldAttack` false)
                (`KismetSystemLibrary.Delay` 3.0)
                (set `self.bShouldGoUp` false)
                (set `self.bShouldGoDown` true)
                (`AudioParameterControllerInterface.SetTriggerParameter` _monster_fightaudio_6 "tWaterSplashDown")
                (`GameplayStatics.SpawnSoundAttached` "/Game/Liam/Audio/Monster/Monster_Audio.Monster_Audio" _monster_fightaudio_6 "None" (0.0 0.0 0.0) (struct) "KeepRelativeOffset" false 1.0 1.0 0.0 null null)
                (`KismetSystemLibrary.Delay` 2.0)
                (set `self.inLoop` false))))))
      (:`then_1`
        (if (not (`self.bIsDead`))
          (`SceneComponent.K2_SetWorldLocation` (`self.HeadCollider`) (.location (`SkinnedMeshComponent.GetBoneTransform` _skeletalmeshseamonster "head1" "RTS_World")) false true)
          (`SceneComponent.K2_SetWorldLocation` (`self.BodyCollider`) (.location (`SkinnedMeshComponent.GetBoneTransform` _skeletalmeshseamonster "spine_base" "RTS_World")) false true))))))

(event `LetMonsterDie`
  (if (not (`KismetSystemLibrary.IsDedicatedServer`))
    (`KismetSystemLibrary.PrintString` "Sea monster will die")
    (set `self.ShouldDie` true)))

(event `SetAttackPattern`
  (params (AttackPattern :type "Array of Integer"))
  (set `self.AttackPattern` AttackPattern)
  (set `self.AttackPatternIndex` 0))

(fn `DeathStateCheck`
  (if (`self.ShouldDie`)
    (set `self.bIsDead` true)
    (set `self.ShouldDie` false)))

(fn `UserConstructionScript`)