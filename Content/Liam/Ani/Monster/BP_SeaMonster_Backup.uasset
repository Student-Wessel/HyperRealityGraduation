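; Backup sea monster boss actor that plays a scripted fight intro on BeginPlay.
; A Delay chain toggles animation state flags, fades an alert material in and out, and fires MonsterFightAudio triggers for splashes, entrance and attack.
; The repeating attack loop with random teleports, bone-following head and body colliders, and editor death toggle is disconnected, as Tick is empty.
; DeathStateCheck turns the editor toggle into IsDead but is never called here.
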(event `self.ReceiveBeginPlay`
  (bind _monster_fightaudio (`self.Monster_FightAudio`))
  (bind _monster_fightaudio_2 (`self.Monster_FightAudio`))
  (bind _monster_fightaudio_3 (`self.Monster_FightAudio`))
  (bind _monster_fightaudio_4 (`self.Monster_FightAudio`))
  (bind _monster_fightaudio_5 (`self.Monster_FightAudio`))
  (bind _monster_fightaudio_6 (`self.Monster_FightAudio`))
  (`|ExecutionSequence`
    (:`then_0`
      ;[1 1 1] Intro
      (`KismetSystemLibrary.Delay` 1.0)
      (`AudioParameterControllerInterface.SetTriggerParameter` _monster_fightaudio_2 "tMonsterAlert")
      (`GameplayStatics.SpawnSoundAttached` "/Game/Liam/Audio/Monster/Monster_Audio.Monster_Audio" _monster_fightaudio_2 "None" (0.0 0.0 0.0) (struct) "KeepRelativeOffset" false 1.0 1.0 0.0 null null)
      (`KismetSystemLibrary.Delay` 2.0)
      (set `self.bStart` true)
      (set `self.fAlertMat_Opacity` 0.4)
      (`MeshComponent.SetScalarParameterValueOnMaterials` (`self.Monster_Alert1`) "Opacity" (`self.fAlertMat_Opacity`))
      (`AudioParameterControllerInterface.SetTriggerParameter` _monster_fightaudio "tWaterSplashUp")
      (`GameplayStatics.SpawnSoundAttached` "/Game/Liam/Audio/Monster/Monster_Audio.Monster_Audio" _monster_fightaudio "None" (0.0 0.0 0.0) (struct) "KeepRelativeOffset" false 1.0 1.0 0.0 null null)
      (`KismetSystemLibrary.Delay` 2.5)
      (`AudioParameterControllerInterface.SetTriggerParameter` _monster_fightaudio_6 "tWaterSplashDown")
      (`GameplayStatics.SpawnSoundAttached` "/Game/Liam/Audio/Monster/Monster_Audio.Monster_Audio" _monster_fightaudio_6 "None" (0.0 0.0 0.0) (struct) "KeepRelativeOffset" false 1.0 1.0 0.0 null null)
      (`KismetSystemLibrary.Delay` 1.0)
      (set `self.fAlertMat_Opacity` 0.0)
      (`MeshComponent.SetScalarParameterValueOnMaterials` (`self.Monster_Alert1`) "Opacity" (`self.fAlertMat_Opacity`))
      (`AudioParameterControllerInterface.SetTriggerParameter` _monster_fightaudio_3 "tMonsterEntrance")
      (`GameplayStatics.SpawnSoundAttached` "/Game/Liam/Audio/Monster/Monster_Audio.Monster_Audio" _monster_fightaudio_3 "None" (0.0 0.0 0.0) (struct) "KeepRelativeOffset" false 1.0 1.0 0.0 null null)
      (`KismetSystemLibrary.Delay` 7.0)
      (`KismetSystemLibrary.DelayUntilNextTick`)
      (set `self.bShouldJump` false)
      (set `self.bShouldGoDown` false)
      (set `self.bShouldAttack` true)
      (`AudioParameterControllerInterface.SetTriggerParameter` _monster_fightaudio_4 "tMonsterAttack")
      (`GameplayStatics.SpawnSoundAttached` "/Game/Liam/Audio/Monster/Monster_Audio.Monster_Audio" _monster_fightaudio_4 "None" (0.0 0.0 0.0) (struct) "KeepRelativeOffset" false 1.0 1.0 0.0 null null)
      (`KismetSystemLibrary.DelayUntilNextTick`)
      (set `self.bShouldAttack` false)
      (`KismetSystemLibrary.Delay` 8.0)
      (set `self.bShouldGoDown` true)
      (`AudioParameterControllerInterface.SetTriggerParameter` _monster_fightaudio_5 "tWaterSplashDown")
      (`GameplayStatics.SpawnSoundAttached` "/Game/Liam/Audio/Monster/Monster_Audio.Monster_Audio" _monster_fightaudio_5 "None" (0.0 0.0 0.0) (struct) "KeepRelativeOffset" false 1.0 1.0 0.0 null null)
      (set `self.inLoop` false))))

(event `self.ReceiveTick`
  (params (DeltaSeconds :type "Float (single-precision)")))

(fn `DeathStateCheck`
  (if (`self.DoEditorDeath`)
    (set `self.bIsDead` true)
    (set `self.DoEditorDeath` false)))

(fn `UserConstructionScript`)