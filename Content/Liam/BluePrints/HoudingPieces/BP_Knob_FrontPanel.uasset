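; Front-panel knob Blueprint for a combination puzzle in which several valves or knobs must each be set to a correct value.
; Every tick it maps CurrentValue from a 1–1023 input range onto the knob mesh's yaw and sets IsCorrect on an exact match with CorrectValue.
; It then checks IsCorrect across an array of elements, stopping at the first failure; the combination result is only printed as debug text.
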(event `self.ReceiveTick`
  (params (DeltaSeconds :type "Float (single-precision)"))
  (`SceneComponent.K2_SetRelativeRotation` (`self.Stuff_02_V01_low_Rotator01_low`) (`KismetMathLibrary.MakeRotator` 0.0 0.0 (`KismetMathLibrary.MapRangeClamped` (`self.currentValue`) 1.0 1023.0 0.0 (`self.Out Range B`))) false false)
  (`KismetSystemLibrary.PrintString` (`KismetStringLibrary.Conv_DoubleToString` (`self.currentValue`)))
  (`self.isValueCorrect`)
  (`self.correctCombo`))

(fn `correctCombo`
  (set `self.allValvesCorrect` true)
  (for _array_element _
    (if (not (`/Game/Bo/Scripts/Valves/BP_Base_Valve.isCorrect` _array_element))
      (`KismetSystemLibrary.PrintString` "False")
      (set `self.allValvesCorrect` false)
      (break)))
  (if (`self.allValvesCorrect`)
    (`KismetSystemLibrary.PrintString` "Correct!")))

(fn `isValueCorrect`
  (bind _returnvalue (`KismetStringLibrary.Conv_BoolToString` (`self.isCorrect`)))
  (if (== (`self.currentValue`) (`self.correctValue`))
    (set `self.isCorrect` true)
    (`KismetSystemLibrary.PrintString` _returnvalue)
    (else
      (set `self.isCorrect` false)
      (`KismetSystemLibrary.PrintString` _returnvalue)))
  (return))

(fn `UserConstructionScript`)