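; Front desk set piece that powers up on interaction and shows feedback for a valve puzzle and a pillar puzzle.
; ValveLights and Pillars check valve and knob actors by index, then multicast material-parameter changes to lamps, screen and pillars.
; Pillar flags are set only on dedicated server and gate the hero light and one-shot roar.
; Each correct knob also triggers MonsterBelow's roar; the gun locker door animation is unconnected.
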(event `self.ReceiveBeginPlay`
  ;[1 0 0] Start_SwitchEmissive_Off
  (`KismetSystemLibrary.Delay` 0.2)
  (set `self.Emissive Switch` 0.0)
  (set `self.ChangeRoofLightColour` 1.0)
  (`MeshComponent.SetScalarParameterValueOnMaterials` (`self.Stuff01_V01_low_Lights_low`) "ChangeToRed" (`self.ChangeRoofLightColour`))
  (bind _outactors (`GameplayStatics.GetAllActorsOfClass` "/Game/Bo/Scripts/Valves/BP_Base_Valve.BP_Base_Valve_C"))
  (set `self.Valves` _outactors)
  (bind _outactors_2 (`GameplayStatics.GetAllActorsOfClass` "/Game/Bo/Scripts/Pillars/BP_Base_Knob.BP_Base_Knob_C"))
  (set `self.Knobs` _outactors_2)
  (bind _returnvalue (`GameplayStatics.GetActorOfClass` "/Game/Chiel/models/monster_v1/MonsterBelow.MonsterBelow_C"))
  (set `self.MonsterBelow` _returnvalue))

(event `Opengunlockers`
  ;[1 1 1] gunlocker
)

(event `Multicast_PlayerMonsterSound`
  (if (not (`KismetSystemLibrary.IsDedicatedServer`))
    (`/Game/Chiel/models/monster_v1/MonsterBelow.PlayMonsterRoaw` (`self.MonsterBelow`))))

(event `/Game/Bo/Scripts/BPI_StartInteraction.Interaction`
  ;[1 1 1] Start
  (`self.Multicast_Delay2`))

(event `/Game/Bo/Scripts/BPI_PuzzleSequences.Pillars`
  (params (rotateIndex :type Integer))
  ;[0.2355 1 0] Puzzle2
  ;;[1 1 1] Checking index
  (`self.Multicast_LowDeskEmissiveSwitch`)
  (for _array_element (`self.Knobs`)
    (if (`/Game/Bo/Scripts/Pillars/BP_Base_Knob.isCorrect` _array_element)
      (bind _rotatorindex (`/Game/Bo/Scripts/Pillars/BP_Base_Knob.rotatorIndex` _array_element))
      (switch `int` _rotatorindex
        (:`0`
          (`self.Multicast_Event_PillarPuzzle01_Correct`))
        (:`1`
          (`self.Multicast_Event_PillarPuzzle02_Correct`))
        (:`2`
          (`self.Multicast_Event_PillarPuzzle03_Correct`))
        (:`3`
          (`self.Multicast_Event_PillarPuzzle04_Correct`)))
      (`self.Puzzle2Correct`)
      (`self.Multicast_PlayerMonsterSound`)
      (else
        (switch `int` _rotatorindex
          (:`0`
            (`self.Multicast_Event_PillarPuzzle01_Incorrect`))
          (:`1`
            (`self.Multicast_Event_PillarPuzzle02_Incorrect`))
          (:`2`
            (`self.Multicast_Event_PillarPuzzle03_Incorrect`))
          (:`3`
            (`self.Multicast_Event_PillarPuzzle04_Incorrect`)))))))

(event `/Game/Bo/Scripts/BPI_PuzzleSequences.ValveLights`
  ;[0.9817 1 0] Puzzle1
  ;;[1 1 1] Checking index
  (for _array_element (`self.Valves`)
    (if (`/Game/Bo/Scripts/Valves/BP_Base_Valve.isCorrect` _array_element)
      (bind _valveindex (`/Game/Bo/Scripts/Valves/BP_Base_Valve.valveIndex` _array_element))
      (switch `int` _valveindex
        (:`0`
          (`self.Multicast_VavleCorrect_01`))
        (:`1`
          (`self.Multicast_VavleCorrect_02`))
        (:`2`
          (`self.Multicast_VavleCorrect_03`))
        (:`3`
          (`self.Multicast_VavleCorrect_04`)))
      (else
        (switch `int` _valveindex
          (:`0`
            (`self.Multicast_ValveIncorrect_01`))
          (:`1`
            (`self.Multicast_ValveIncorrect_02`))
          (:`2`
            (`self.Multicast_ValveIncorrect_3`))
          (:`3`
            (`self.Multicast_ValveIncorrect_4`)))))))

(event `Multicast_Delay2`
  (bind _emissive_switch (`self.Emissive Switch`))
  ;[1 1 1] Start
  ;;[1 1 1] Handscanners_Pressed
  (if (not (`KismetSystemLibrary.IsDedicatedServer`))
    (set `self.Emissive Switch` 1.0)
    (set `self.ChangeRoofLightColour` 0.0)
    ;;[1 1 1] FrontPanel_Emissive_Switch
    (`MeshComponent.SetScalarParameterValueOnMaterials` (`self.Stuff_02_V01_low_Desk02_low`) "Emissive_Switch" _emissive_switch)
    (`MeshComponent.SetScalarParameterValueOnMaterials` (`self.Stuff_02_V01_low_GunLocker_low`) "Emissive_Switch" _emissive_switch)
    (`MeshComponent.SetScalarParameterValueOnMaterials` (`self.Stuff_02_V01_low_GunLockerDoor_low`) "Emissive_Switch" _emissive_switch)
    (`MeshComponent.SetScalarParameterValueOnMaterials` (`self.Stuff_02_V01_low_GunLockerDoor_low1`) "Emissive_Switch" _emissive_switch)
    (`MeshComponent.SetScalarParameterValueOnMaterials` (`self.Stuff_02_V01_low_GunLocker_low1`) "Emissive_Switch" _emissive_switch)
    ;;[1 1 1] Handscanner
    (`MeshComponent.SetScalarParameterValueOnMaterials` (`self.Stuff_02_V01_low_Scanner_low`) "Emissive_Switch" _emissive_switch)
    (`MeshComponent.SetScalarParameterValueOnMaterials` (`self.Stuff_02_V01_low_Scanner_low1`) "Emissive_Switch" _emissive_switch)
    ;;[1 1 1] Left_Panel
    (`MeshComponent.SetScalarParameterValueOnMaterials` (`self.Stuff_02_V01_low_DeskScreen_low`) "Emissive_Switch" _emissive_switch)
    (`MeshComponent.SetScalarParameterValueOnMaterials` (`self.Stuff02_Desk01_IncludingScreen_Desk01_low`) "Emissive_Switch" _emissive_switch)
    ;;[1 1 1] Pipe_Lights
    (`MeshComponent.SetScalarParameterValueOnMaterials` (`self.Stuff_02_V01_low_WallLamp_01`) "Emissive_Switch" _emissive_switch)
    (`MeshComponent.SetScalarParameterValueOnMaterials` (`self.Stuff_02_V01_low_WallLamp_02`) "Emissive_Switch" _emissive_switch)
    (`MeshComponent.SetScalarParameterValueOnMaterials` (`self.Stuff_02_V01_low_WallLamp_03`) "Emissive_Switch" _emissive_switch)
    (`MeshComponent.SetScalarParameterValueOnMaterials` (`self.Stuff_02_V01_low_WallLamp_04`) "Emissive_Switch" _emissive_switch)
    ;;[1 1 1] RoofLights
    (`MeshComponent.SetScalarParameterValueOnMaterials` (`self.Stuff01_V01_low_Lights_low`) "ChangeToRed" (`self.ChangeRoofLightColour`))))

(event `Multicast_LowDeskEmissiveSwitch`
  ;[0.2355 1 0] Puzzle2
  ;;[1 1 1] Checking index
  (set `self.Emissive Switch` 1.0)
  (`MeshComponent.SetScalarParameterValueOnMaterials` (`self.Stuff_02_V01_low_DeskScreen_low`) "Emissive_Switch" (`self.Emissive Switch`)))

(event `Multicast_Event_PillarPuzzle01_Correct`
  ;[0.2355 1 0] Puzzle2
  ;;[1 1 1] LeftPuzzle(On)
  ;;;[1 1 1] Puzzle01_On
  (if (`KismetSystemLibrary.IsDedicatedServer`)
    (set `self.PillarPuzzle01_Correct` true)
    (else
      (set `self.01Screen_Switch` 1.0)
      (`MeshComponent.SetScalarParameterValueOnMaterials` (`self.Stuff_02_V01_low_DeskScreen_low`) "01_Correct" (`self.01Screen_Switch`))
      (set `self.01Pillar_Switch` 10.0)
      (`MeshComponent.SetScalarParameterValueOnMaterials` (`self.Pillars_Sq_Hyro_01`) "Emissive_Intensity" (`self.01Pillar_Switch`)))))

(event `Multicast_Event_PillarPuzzle01_Incorrect`
  ;[0.2355 1 0] Puzzle2
  ;;[1 1 1] LeftPuzzle(Off)
  ;;;[1 1 1] Puzzle01_Off
  (if (`KismetSystemLibrary.IsDedicatedServer`)
    (set `self.PillarPuzzle01_Correct` false)
    (else
      (set `self.01Screen_Switch` 0.0)
      (`MeshComponent.SetScalarParameterValueOnMaterials` (`self.Stuff_02_V01_low_DeskScreen_low`) "01_Correct" (`self.01Screen_Switch`))
      (set `self.01Pillar_Switch` 0.0)
      (`MeshComponent.SetScalarParameterValueOnMaterials` (`self.Pillars_Sq_Hyro_01`) "Emissive_Intensity" (`self.01Pillar_Switch`)))))

(event `Multicast_ValveIncorrect_01`
  ;[0.9817 1 0] Puzzle1
  ;;[1 1 1] TurnValves(Off)
  ;;;[1 1 1] Vavle_01_Off
  (if (not (`KismetSystemLibrary.IsDedicatedServer`))
    (set `self.ValveLight` 0.0)
    (`MeshComponent.SetScalarParameterValueOnMaterials` (`self.Stuff_02_V01_low_WallLamp_01`) "Turn_Green" (`self.ValveLight`))))

(event `Multicast_VavleCorrect_01`
  ;[0.9817 1 0] Puzzle1
  ;;[1 1 1] TurnValves(On)
  ;;;[1 1 1] Vavle_01_On
  (if (not (`KismetSystemLibrary.IsDedicatedServer`))
    (set `self.ValveLight` 1.0)
    (`MeshComponent.SetScalarParameterValueOnMaterials` (`self.Stuff_02_V01_low_WallLamp_01`) "Turn_Green" (`self.ValveLight`))))

(event `Multicast_ValveIncorrect_02`
  ;[0.9817 1 0] Puzzle1
  ;;[1 1 1] TurnValves(Off)
  ;;;[1 1 1] Vavle_02_Off
  (if (not (`KismetSystemLibrary.IsDedicatedServer`))
    (set `self.ValveLight` 0.0)
    (`MeshComponent.SetScalarParameterValueOnMaterials` (`self.Stuff_02_V01_low_WallLamp_02`) "Turn_Green" (`self.ValveLight`))))

(event `Multicast_VavleCorrect_02`
  ;[0.9817 1 0] Puzzle1
  ;;[1 1 1] TurnValves(On)
  ;;;[1 1 1] Vavle_02_On
  (if (not (`KismetSystemLibrary.IsDedicatedServer`))
    (set `self.ValveLight` 1.0)
    (`MeshComponent.SetScalarParameterValueOnMaterials` (`self.Stuff_02_V01_low_WallLamp_02`) "Turn_Green" (`self.ValveLight`))))

(event `Multicast_Event_PillarPuzzle02_Correct`
  ;[0.9817 1 0] Puzzle1
  ;[0.2355 1 0] Puzzle2
  ;;[1 1 1] LeftPuzzle(On)
  ;;;[1 1 1] Puzzle02_On
  (if (`KismetSystemLibrary.IsDedicatedServer`)
    (set `self.PillarPuzzle02_Correct` true)
    (else
      (set `self.02Screen_Switch` 1.0)
      (`MeshComponent.SetScalarParameterValueOnMaterials` (`self.Stuff_02_V01_low_DeskScreen_low`) "02_Correct" (`self.02Screen_Switch`))
      (set `self.02Pillar_Switch` 10.0)
      (`MeshComponent.SetScalarParameterValueOnMaterials` (`self.Pillars_Sq_Hyro_02`) "Emissive_Intensity" (`self.02Pillar_Switch`)))))

(event `Multicast_Event_PillarPuzzle02_Incorrect`
  ;[0.2355 1 0] Puzzle2
  ;;[1 1 1] LeftPuzzle(Off)
  ;;;[1 1 1] Puzzle02_Off
  (if (`KismetSystemLibrary.IsDedicatedServer`)
    (set `self.PillarPuzzle02_Correct` false)
    (else
      (set `self.02Screen_Switch` 0.0)
      (`MeshComponent.SetScalarParameterValueOnMaterials` (`self.Stuff_02_V01_low_DeskScreen_low`) "02_Correct" (`self.02Screen_Switch`))
      (set `self.02Pillar_Switch` 0.0)
      (`MeshComponent.SetScalarParameterValueOnMaterials` (`self.Pillars_Sq_Hyro_02`) "Emissive_Intensity" (`self.02Pillar_Switch`)))))

(event `Multicast_ValveIncorrect_3`
  ;[1 1 1] Start
  ;[0.9817 1 0] Puzzle1
  ;;[1 1 1] TurnValves(Off)
  ;;;[1 1 1] Vavle_03_Off
  (if (not (`KismetSystemLibrary.IsDedicatedServer`))
    (set `self.ValveLight` 0.0)
    (`MeshComponent.SetScalarParameterValueOnMaterials` (`self.Stuff_02_V01_low_WallLamp_03`) "Turn_Green" (`self.ValveLight`))))

(event `Multicast_VavleCorrect_03`
  ;[0.9817 1 0] Puzzle1
  ;;[1 1 1] TurnValves(On)
  ;;;[1 1 1] Vavle_03_On
  (if (not (`KismetSystemLibrary.IsDedicatedServer`))
    (set `self.ValveLight` 1.0)
    (`MeshComponent.SetScalarParameterValueOnMaterials` (`self.Stuff_02_V01_low_WallLamp_03`) "Turn_Green" (`self.ValveLight`))))

(event `Multicast_Event_PillarPuzzle03_Correct`
  ;[0.9817 1 0] Puzzle1
  ;[0.2355 1 0] Puzzle2
  ;;[1 1 1] LeftPuzzle(On)
  ;;;[1 1 1] Puzzle03_On
  (if (`KismetSystemLibrary.IsDedicatedServer`)
    (set `self.PillarPuzzle03_Correct` true)
    (else
      (set `self.03Screen_Switch` 1.0)
      (`MeshComponent.SetScalarParameterValueOnMaterials` (`self.Stuff_02_V01_low_DeskScreen_low`) "03_Correct" (`self.03Screen_Switch`))
      (set `self.03Pillar_Switch` 10.0)
      (`MeshComponent.SetScalarParameterValueOnMaterials` (`self.Pillars_Sq_Hyro_03`) "Emissive_Intensity" (`self.03Pillar_Switch`)))))

(event `Multicast_Event_PillarPuzzle03_Incorrect`
  ;[0.2355 1 0] Puzzle2
  ;;[1 1 1] LeftPuzzle(Off)
  ;;;[1 1 1] Puzzle03_Off
  (if (`KismetSystemLibrary.IsDedicatedServer`)
    (set `self.PillarPuzzle03_Correct` false)
    (else
      (set `self.03Screen_Switch` 0.0)
      (`MeshComponent.SetScalarParameterValueOnMaterials` (`self.Stuff_02_V01_low_DeskScreen_low`) "03_Correct" (`self.03Screen_Switch`))
      (set `self.03Pillar_Switch` 0.0)
      (`MeshComponent.SetScalarParameterValueOnMaterials` (`self.Pillars_Sq_Hyro_03`) "Emissive_Intensity" (`self.03Pillar_Switch`)))))

(event `Multicast_ValveIncorrect_4`
  ;[0.9817 1 0] Puzzle1
  ;;[1 1 1] TurnValves(Off)
  ;;;[1 1 1] Vavle_04_Off
  (if (not (`KismetSystemLibrary.IsDedicatedServer`))
    (set `self.ValveLight` 0.0)
    (`MeshComponent.SetScalarParameterValueOnMaterials` (`self.Stuff_02_V01_low_WallLamp_04`) "Turn_Green" (`self.ValveLight`))))

(event `Multicast_VavleCorrect_04`
  ;[0.9817 1 0] Puzzle1
  ;;[1 1 1] TurnValves(On)
  ;;;[1 1 1] Vavle_04_On
  (if (not (`KismetSystemLibrary.IsDedicatedServer`))
    (set `self.ValveLight` 1.0)
    (`MeshComponent.SetScalarParameterValueOnMaterials` (`self.Stuff_02_V01_low_WallLamp_04`) "Turn_Green" (`self.ValveLight`))))

(event `Multicast_Event_PillarPuzzle04_Correct`
  ;[0.9817 1 0] Puzzle1
  ;[0.2355 1 0] Puzzle2
  ;;[1 1 1] LeftPuzzle(On)
  ;;;[1 1 1] Puzzle04_On
  (if (`KismetSystemLibrary.IsDedicatedServer`)
    (set `self.PillarPuzzle04_Correct` true)
    (else
      (set `self.04Screen_Switch` 1.0)
      (`MeshComponent.SetScalarParameterValueOnMaterials` (`self.Stuff_02_V01_low_DeskScreen_low`) "04_Correct" (`self.04Screen_Switch`))
      (set `self.04Pillar_Switch` 10.0)
      (`MeshComponent.SetScalarParameterValueOnMaterials` (`self.Pillars_Sq_Hyro_04`) "Emissive_Intensity" (`self.04Pillar_Switch`)))))

(event `Multicast_Event_PillarPuzzle04_Incorrect`
  ;[0.2355 1 0] Puzzle2
  ;;[1 1 1] LeftPuzzle(Off)
  ;;;[1 1 1] Puzzle04_Off
  (if (`KismetSystemLibrary.IsDedicatedServer`)
    (set `self.PillarPuzzle04_Correct` false)
    (else
      (set `self.04Screen_Switch` 0.0)
      (`MeshComponent.SetScalarParameterValueOnMaterials` (`self.Stuff_02_V01_low_DeskScreen_low`) "04_Correct" (`self.04Screen_Switch`))
      (set `self.04Pillar_Switch` 0.0)
      (`MeshComponent.SetScalarParameterValueOnMaterials` (`self.Pillars_Sq_Hyro_04`) "Emissive_Intensity" (`self.04Pillar_Switch`)))))

(event `Puzzle2Correct`
  ;[0.2355 1 0] Puzzle2
  ;;[1 1 1] Comment
  (if (and (`self.PillarPuzzle01_Correct`) (`self.PillarPuzzle02_Correct`) (`self.PillarPuzzle03_Correct`) (`self.PillarPuzzle04_Correct`))
    ;;;[1 1 1] PuzzleHero_On
    (set `self.05HeroScreen_Switch` 1.0)
    (`MeshComponent.SetScalarParameterValueOnMaterials` (`self.Stuff_02_V01_low_DeskScreen_low`) "05_Correct_Mid" (`self.05HeroScreen_Switch`))
    (set `self.05HeroPillar_Switch` 10.0)
    (`MeshComponent.SetScalarParameterValueOnMaterials` (`self.Hero_Pillar_SD`) "Emissive_Intensity" (`self.05HeroPillar_Switch`))
    (set `self.PillarPuzzle_Finished` true)
    (`/Engine/EditorBlueprintResources/StandardMacros.DoOnce` false
      (:`Completed`
        (`GameplayStatics.PlaySoundAtLocation` "/Game/Bo/Test/MonsterConcept_Distant_Roar_1_V1.MonsterConcept_Distant_Roar_1_V1" (0.0 0.0 0.0) (struct) 1.0 1.0 0.0 null null null null)))
    (else
      ;;;[1 1 1] PuzzleHero_Off
      (set `self.05HeroScreen_Switch` 0.0)
      (`MeshComponent.SetScalarParameterValueOnMaterials` (`self.Stuff_02_V01_low_DeskScreen_low`) "05_Correct_Mid" (`self.05HeroScreen_Switch`))
      (set `self.05HeroPillar_Switch` 0.0)
      (`MeshComponent.SetScalarParameterValueOnMaterials` (`self.Hero_Pillar_SD`) "Emissive_Intensity" (`self.05HeroPillar_Switch`))
      (set `self.PillarPuzzle_Finished` false))))

(event `Multicast_Puzzle2CorrectNotify`)

(event `Multicast_Puzzle2IncorrectNotify`)

(fn `UserConstructionScript`
  (locals (NewLocalVar :type "Float (double-precision)" :default 0.0))
  (set `self.Emissive Switch` 0.0)
  (`MeshComponent.SetScalarParameterValueOnMaterials` (`self.Stuff_02_V01_low_DeskScreen_low`) "Emissive_Switch" (`self.Emissive Switch`))
  (set `self.ValveLight` 0.0)
  (`MeshComponent.SetScalarParameterValueOnMaterials` (`self.Stuff_02_V01_low_WallLamp_01`) "Turn_Green" (`self.ValveLight`))
  (set `self.ChangeRoofLightColour` 0.0)
  (`MeshComponent.SetScalarParameterValueOnMaterials` (`self.Stuff01_V01_low_Lights_low`) "ChangeToRed" (`self.ChangeRoofLightColour`))
  (set `self.01Pillar_Switch` 0.0)
  (set `self.02Pillar_Switch` 0.0)
  (set `self.03Pillar_Switch` 0.0)
  (set `self.04Pillar_Switch` 0.0)
  (set `self.05HeroPillar_Switch` 0.0)
  (`MeshComponent.SetScalarParameterValueOnMaterials` (`self.Pillars_Sq_Hyro_01`) "Emissive_Intensity" (`self.01Pillar_Switch`))
  (`MeshComponent.SetScalarParameterValueOnMaterials` (`self.Pillars_Sq_Hyro_02`) "Emissive_Intensity" (`self.02Pillar_Switch`))
  (`MeshComponent.SetScalarParameterValueOnMaterials` (`self.Pillars_Sq_Hyro_03`) "Emissive_Intensity" (`self.03Pillar_Switch`))
  (`MeshComponent.SetScalarParameterValueOnMaterials` (`self.Pillars_Sq_Hyro_04`) "Emissive_Intensity" (`self.04Pillar_Switch`))
  (`MeshComponent.SetScalarParameterValueOnMaterials` (`self.Hero_Pillar_SD`) "Emissive_Intensity" (`self.05HeroPillar_Switch`))
  (set `self.01Screen_Switch` 0.0)
  (set `self.02Screen_Switch` 0.0)
  (set `self.03Screen_Switch` 0.0)
  (set `self.04Screen_Switch` 0.0)
  (set `self.05HeroScreen_Switch` 0.0)
  (`MeshComponent.SetScalarParameterValueOnMaterials` (`self.Stuff_02_V01_low_DeskScreen_low`) "01_Correct" (`self.01Screen_Switch`))
  (`MeshComponent.SetScalarParameterValueOnMaterials` (`self.Stuff_02_V01_low_DeskScreen_low`) "02_Correct" (`self.02Screen_Switch`))
  (`MeshComponent.SetScalarParameterValueOnMaterials` (`self.Stuff_02_V01_low_DeskScreen_low`) "03_Correct" (`self.03Screen_Switch`))
  (`MeshComponent.SetScalarParameterValueOnMaterials` (`self.Stuff_02_V01_low_DeskScreen_low`) "04_Correct" (`self.04Screen_Switch`))
  (`MeshComponent.SetScalarParameterValueOnMaterials` (`self.Stuff_02_V01_low_DeskScreen_low`) "05_Correct_Mid" (`self.05HeroScreen_Switch`))
  (set `self.PillarPuzzle01_Correct` false)
  (set `self.PillarPuzzle02_Correct` false)
  (set `self.PillarPuzzle03_Correct` false)
  (set `self.PillarPuzzle04_Correct` false)
  (set `self.PillarPuzzle_Finished` false))