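; Elevator shutter actor whose OpenShutters event slides two panels apart to open.
; A sequence starts two timelines together, each lerping one panel from the root's location toward an opposite, unequal offset on world Y, so the motion ignores actor rotation.
; Each timeline ends in a short delay with nothing after it, and the file has no closing logic.
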(event `OpenShutters`
  (bind _defaultsceneroot (`self.DefaultSceneRoot`))
  (bind _defaultsceneroot_2 (`self.DefaultSceneRoot`))
  (bind (_returnvalue_x _returnvalue_y _returnvalue_z) (`KismetMathLibrary.BreakVector` (`SceneComponent.K2_GetComponentLocation` _defaultsceneroot_2)))
  (bind (_returnvalue_x_2 _returnvalue_y_2 _returnvalue_z_2) (`KismetMathLibrary.BreakVector` (`SceneComponent.K2_GetComponentLocation` _defaultsceneroot)))
  (`|ExecutionSequence`
    (:`then_0`
      (bind (_direction _newtrack_0) (`Timeline|Timeline` :!via `PlayFromStart`)
        (:`Update`
          (`SceneComponent.K2_SetWorldLocation` (`self.Panel1`) (`KismetMathLibrary.VLerp` (`SceneComponent.K2_GetComponentLocation` _defaultsceneroot) (`KismetMathLibrary.MakeVector` _returnvalue_x_2 (- _returnvalue_y_2 120.0) _returnvalue_z_2) _newtrack_0) false false))
        (:`Finished`
          (`KismetSystemLibrary.Delay` 1.0))))
    (:`then_1`
      (bind (_direction_2 _newtrack_0_2) (`Timeline|Timeline_0` :!via `PlayFromStart`)
        (:`Update`
          (`SceneComponent.K2_SetWorldLocation` (`self.Panel2`) (`KismetMathLibrary.VLerp` (`SceneComponent.K2_GetComponentLocation` _defaultsceneroot_2) (`KismetMathLibrary.MakeVector` _returnvalue_x (+ _returnvalue_y 100.0) _returnvalue_z) _newtrack_0_2) false false))
        (:`Finished`
          (`KismetSystemLibrary.Delay` 1.0))))))

(fn `UserConstructionScript`)