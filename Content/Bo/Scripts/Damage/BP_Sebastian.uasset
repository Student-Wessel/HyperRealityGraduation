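; BP_Sebastian is a boss-style monster that cycles through relocating, rising, attacking and descending.
; BeginPlay runs a timed intro, then Tick drives a delay-based loop gated by InLoop until zero health sets IsDead.
; MonsterPosition moves it using random picks from BTeleportPositions, re-rolled inside a loop over the array.
; AnimState maps the attack, up, down and death flags to an animation enum, with death sharing the descend state.
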(event `self.ReceiveBeginPlay`
  ;[1 1 1] Intro
  (`KismetSystemLibrary.Delay` 1.0)
  (set `self.bShouldJump` true)
  (`KismetSystemLibrary.Delay` 4.0)
  (set `self.bShouldJump` false)
  (set `self.bStart` true)
  (`|ExecutionSequence`
    (:`then_0`
      (set `self.bShouldGoDown` false))
    (:`then_1`
      (set `self.bShouldGoUp` false))
    (:`then_2`
      (set `self.bShouldAttack` true)
      (`KismetSystemLibrary.DelayUntilNextTick`)
      (set `self.bShouldAttack` false)
      (`KismetSystemLibrary.Delay` 6.0)
      (set `self.bShouldGoDown` true)
      (set `self.inLoop` false))))

(event `self.ReceiveTick`
  (params (DeltaSeconds :type "Float (single-precision)"))
  (`|ExecutionSequence`
    (:`then_0`
      (if (`self.inLoop`)
        _
        (elif (== (`self.bIsDead`) false)
          (set `self.inLoop` true)
          (`KismetSystemLibrary.Delay` 1.0)
          (`self.Event MonsterPosition`)
          (set `self.bShouldGoDown` false)
          (set `self.bShouldGoUp` true)
          (`KismetSystemLibrary.Delay` 3.0)
          (set `self.bShouldAttack` true)
          (`KismetSystemLibrary.Delay` 3.0)
          (set `self.bShouldAttack` false)
          (`KismetSystemLibrary.Delay` 6.0)
          (set `self.bShouldGoUp` false)
          (set `self.bShouldGoDown` true)
          (`KismetSystemLibrary.Delay` 2.0)
          (set `self.inLoop` false))))
    (:`then_1`
      (if (== (`self.fHealth`) 0.0)
        (set `self.bShouldJump` true)
        (set `self.bIsDead` true)))))

(event `Event MonsterPosition`
  (bind (_outitem _outindex) (`KismetArrayLibrary.Array_Random` (`self.bTeleportPositions`)))
  (bind (_position _rotation) (break `/Game/Liam/Data_Stucture/S_MonsterLocation` _outitem))
  ;[1 1 1] RandomizedPosition
  (for (_ _array_index) (`self.bTeleportPositions`)
    (bind _returnvalue (== _array_index _outindex))
    (if (not _returnvalue)
      (`self.K2_SetActorLocationAndRotation` _position _rotation)
      (`KismetSystemLibrary.PrintString` (`KismetStringLibrary.Conv_BoolToString` _returnvalue)))))

(fn `AnimState`
  (`|ExecutionSequence`
    (:`then_0`
      (if (`self.bShouldAttack`)
        (set `self.animationState` "NewEnumerator3")))
    (:`then_1`
      (if (`self.bShouldGoUp`)
        (set `self.animationState` "NewEnumerator0")))
    (:`then_2`
      (if (`self.bShouldGoDown`)
        (set `self.animationState` "NewEnumerator1")))
    (:`then_3`
      (if (`self.bIsDead`)
        (set `self.animationState` "NewEnumerator1")))))

(fn `UserConstructionScript`)