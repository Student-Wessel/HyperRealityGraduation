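; BP_Gun is a gun actor with a BulletSpawn component marking the muzzle, but it has no active firing behavior.
; An unconnected chain line-traces between BulletSpawn and a point just ahead, ignores the hit, then spawns a BP_Bullet along the forward vector and destroys it after a short delay.
; Tick and the construction script are empty, and ReturnData ignores its Actor input and returns zero.
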(event `self.ReceiveTick`
  (params (DeltaSeconds :type "Float (single-precision)")))

(fn `ReturnData`
  (params (Actor :type "Actor Object Reference"))
  (returns (Index :type Integer))
  (return 0))

(fn `UserConstructionScript`)