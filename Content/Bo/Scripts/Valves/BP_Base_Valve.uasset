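; Base valve for a multi-valve puzzle, smoothly rotating its mesh on roll toward a scaled value fed through UpdateValue.
; On new values, a dedicated server checks against the correct value within a tolerance and reports only changes in correctness via CallValveCorrectUpdate.
; Otherwise, it plays a random turning sound, gated until the previous one finishes.
; CorrectCombo scans all valves to set whether every one is correct.
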(event `self.ReceiveTick`
  (params (DeltaSeconds :type "Float (single-precision)"))
  ;[1 1 1] Rotate
  (`SceneComponent.K2_SetRelativeRotation` (`self.Valve_0`) (`KismetMathLibrary.RInterpTo` (`SceneComponent.RelativeRotation` (`self.Valve_0`)) (`KismetMathLibrary.MakeRotator` (`self.currentValue`)) DeltaSeconds 5.0) false false)
  (if (`KismetSystemLibrary.IsDedicatedServer`)
    (if (`self.HasNewValue`)
      (set `self.HasNewValue` false)
      (`self.isValueCorrect`))
    (else
      ;[0.3496 0.2723 1] Play a random valve sound everytime
      (if (`self.HasNewValue`)
        (`|ExecutionSequence`
          (:`then_0`
            (set `self.HasNewValue` false))
          (:`then_1`
            (if (`self.CanIPlaySound`)
              (set `self.CanIPlaySound` false)
              (switch `int` (`KismetMathLibrary.RandomInteger` 4)
                (:`0`
                  (`AudioComponent.Play` (`self.SFX_Valve_Rotate0`) 0.0))
                (:`1`
                  (`AudioComponent.Play` (`self.SFX_Valve_Rotate1`) 0.0))
                (:`2`
                  (`AudioComponent.Play` (`self.SFX_Valve_Rotate2`) 0.0))
                (:`3`
                  (`AudioComponent.Play` (`self.SFX_Valve_Rotate3`) 0.0))
                (:`4`
                  (`AudioComponent.Play` (`self.SFX_Valve_Rotate4`) 0.0))))))))))

(event `self.SFX_Valve_Rotate0.OnAudioFinished`
  ;[0.3496 0.2723 1] Play a random valve sound everytime
  (set `self.CanIPlaySound` true :!label _label))

(event `self.SFX_Valve_Rotate1.OnAudioFinished`
  ;[0.3496 0.2723 1] Play a random valve sound everytime
  (goto _label))

(event `self.SFX_Valve_Rotate2.OnAudioFinished`
  ;[0.3496 0.2723 1] Play a random valve sound everytime
  (goto _label))

(event `self.SFX_Valve_Rotate3.OnAudioFinished`
  ;[0.3496 0.2723 1] Play a random valve sound everytime
  (goto _label))

(event `self.SFX_Valve_Rotate4.OnAudioFinished`
  ;[0.3496 0.2723 1] Play a random valve sound everytime
  (goto _label))

(fn `correctCombo`
  (set `self.allValvesCorrect` true)
  (bind _outactors (`GameplayStatics.GetAllActorsOfClass` "BP_Base_Valve_C"))
  (for _array_element _outactors
    (if (not (`/Game/Bo/Scripts/Valves/BP_Base_Valve.isCorrect` _array_element))
      (set `self.allValvesCorrect` false)
      (break))))

(fn `isValueCorrect`
  (if (`KismetMathLibrary.NearlyEqual_FloatFloat` (`KismetMathLibrary.Abs` (`self.currentValue`)) (`self.correctValue`) 25.0)
    (bind _output_get (set `self.isCorrect` true))
    (if (not (`self.PreviousWasCorrect`))
      (set `self.PreviousWasCorrect` true)
      (`self.ValveCorrectUpdate` _output_get))
    (else
      (bind _output_get_2 (set `self.isCorrect` false))
      (if (`self.PreviousWasCorrect`)
        (set `self.PreviousWasCorrect` false)
        (`self.ValveCorrectUpdate` _output_get_2)))))

(fn `ReturnData`
  (returns (Index :type Integer))
  (return 0))

(fn `UpdateValue`
  (params (NewValue :type "Float (double-precision)"))
  (set `self.currentValue` (* NewValue 0.155))
  (set `self.HasNewValue` true))

(fn `UserConstructionScript`)

(fn `ValveData`
  (params (NewParam :type Boolean))
  (return))