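; BP_Shutters is an interactable shutter actor that slides open upward and then removes itself.
; Its Interaction event calls a multicast notify event, which prints debug messages and skips the animation on dedicated servers.
; Elsewhere, a timeline lerps the Shutters component's world position upward from the root, then destroys the actor after a short delay.
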(event `Multicast_NotifyClient`
  (bind (_returnvalue_x _returnvalue_y _returnvalue_z) (`KismetMathLibrary.BreakVector` (`SceneComponent.K2_GetComponentLocation` (`self.DefaultSceneRoot`))))
  (for _ (range 10)
    (`KismetSystemLibrary.PrintString` "Should go open"))
  (if (not (`KismetSystemLibrary.IsDedicatedServer`))
    (bind (_direction _newtrack_0) (`Timeline|Timeline` :!via `PlayFromStart`)
      (:`Update`
        (`SceneComponent.K2_SetWorldLocation` (`self.Shutters`) (`KismetMathLibrary.VLerp` (`SceneComponent.K2_GetComponentLocation` (`self.DefaultSceneRoot`)) (`KismetMathLibrary.MakeVector` _returnvalue_x _returnvalue_y (+ _returnvalue_z 200.0)) _newtrack_0) false false))
      (:`Finished`
        (`KismetSystemLibrary.Delay` 1.0)
        (`self.K2_DestroyActor`)))))

(event `/Game/Bo/Scripts/BPI_StartInteraction.Interaction`
  (`self.Multicast_NotifyClient`)
  (`KismetSystemLibrary.PrintString` "Send Multicast"))

(fn `UserConstructionScript`)