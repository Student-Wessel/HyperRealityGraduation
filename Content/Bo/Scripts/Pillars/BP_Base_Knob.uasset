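; BP_Base_Knob is a puzzle knob that eases its yaw toward a value set by UpdateValue.
; On a dedicated server, Tick handles new values by checking them against an asymmetric window around CorrectValue, reporting the result and playing a random rotate sound.
; Sounds are gated until playback finishes; the fifth is never picked.
; CorrectCombo, not called here, prints when every BP_Base_Valve is correct.
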(event `self.SFX_Knob_Rotate0.OnAudioFinished`
  ;[0.3496 0.2723 1] Play a random valve knob everytime a knob is updated
  (set `self.CanIPlaySound` true :!label _label))

(event `self.SFX_Knob_Rotate1.OnAudioFinished`
  ;[0.3496 0.2723 1] Play a random valve knob everytime a knob is updated
  (goto _label))

(event `self.SFX_Knob_Rotate2.OnAudioFinished`
  ;[0.3496 0.2723 1] Play a random valve knob everytime a knob is updated
  (goto _label))

(event `self.SFX_Knob_Rotate3.OnAudioFinished`
  ;[0.3496 0.2723 1] Play a random valve knob everytime a knob is updated
  (goto _label))

(event `self.SFX_Knob_Rotate4.OnAudioFinished`
  ;[0.3496 0.2723 1] Play a random valve knob everytime a knob is updated
  (goto _label))

(event `self.ReceiveTick`
  (params (DeltaSeconds :type "Float (single-precision)"))
  (bind _knob (`self.knob`))
  (`SceneComponent.K2_SetRelativeRotation` _knob (`KismetMathLibrary.RInterpTo` (`SceneComponent.RelativeRotation` _knob) (`KismetMathLibrary.MakeRotator` 0.0 0.0 (`self.currentValue`)) DeltaSeconds 5.0) false false)
  (if (`KismetSystemLibrary.IsDedicatedServer`)
    (if (`self.HasNewValue`)
      ;[0.3496 0.2723 1] Play a random valve knob everytime a knob is updated
      (`|ExecutionSequence`
        (:`then_0`
          (set `self.HasNewValue` false)
          (`self.isValueCorrect`))
        (:`then_1`
          (if (`self.CanIPlaySound`)
            (set `self.CanIPlaySound` false)
            (switch `int` (`KismetMathLibrary.RandomInteger` 4)
              (:`0`
                (`AudioComponent.Play` (`self.SFX_Knob_Rotate0`) 0.0))
              (:`1`
                (`AudioComponent.Play` (`self.SFX_Knob_Rotate1`) 0.0))
              (:`2`
                (`AudioComponent.Play` (`self.SFX_Knob_Rotate2`) 0.0))
              (:`3`
                (`AudioComponent.Play` (`self.SFX_Knob_Rotate3`) 0.0))
              (:`4`
                (`AudioComponent.Play` (`self.SFX_Knob_Rotate4`) 0.0)))))))))

(fn `correctCombo`
  (set `self.allRotatorCorrect` true)
  (bind _outactors (`GameplayStatics.GetAllActorsOfClass` "/Game/Bo/Scripts/Valves/BP_Base_Valve.BP_Base_Valve_C"))
  (for _array_element _outactors
    (if (not (`/Game/Bo/Scripts/Valves/BP_Base_Valve.isCorrect` _array_element))
      (set `self.allRotatorCorrect` false)
      (break)))
  (if (`self.allRotatorCorrect`)
    (`KismetSystemLibrary.PrintString` "Correct!")))

(fn `isValueCorrect`
  (bind _currentvalue (`self.currentValue`))
  (if (and (>= _currentvalue (- (`self.correctValue`) 10.0)) (<= _currentvalue (+ (`self.correctValue`) 50.0)))
    (bind _output_get (set `self.isCorrect` true))
    (`self.ValueCorrectUpdate` _output_get)
    (else
      (bind _output_get_2 (set `self.isCorrect` false))
      (`self.ValueCorrectUpdate` _output_get_2))))

(fn `UpdateValue`
  (params (NewValue :type "Float (double-precision)"))
  (set `self.currentValue` NewValue)
  (set `self.HasNewValue` true))

(fn `UserConstructionScript`)